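; BP_SteamingVent is a smoking vent prop that gets knocked loose when something first overlaps its trigger box.
; The overlap enables physics, launches the vent along a normalized, actor-relative Impulse direction, destroys the box and disables the Smoke emitter.
; A looping timer then polls the vent's velocity, and once it is zero stops simulation, clears itself and destroys the particle component.
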(event `self.Box.OnComponentBeginOverlap`
  (params (OverlappedComponent :type "PrimitiveComponent Object Reference") (OtherActor :type "Actor Object Reference") (OtherComp :type "PrimitiveComponent Object Reference") (OtherBodyIndex :type Integer) (bFromSweep :type Boolean) (SweepResult :type "HitResult Structure (by ref)"))
  (bind _vent (`self.Vent`))
  (`PrimitiveComponent.SetSimulatePhysics` _vent true)
  (`PrimitiveComponent.AddImpulse` _vent (* (`KismetMathLibrary.Normal` (`KismetMathLibrary.TransformDirection` (`self.GetTransform`) (`self.Impulse`))) 5000.0) "None" false)
  (`ActorComponent.K2_DestroyComponent` (`self.Box`))
  (`FXSystemComponent.SetEmitterEnable` (`self.VentilationParticles`) "Smoke" false)
  (bind _returnvalue (`KismetSystemLibrary.K2_SetTimerDelegate` (delegate `StopSimulating`) 2.0 true))
  (set `self.SimTimer` _returnvalue))

(event `StopSimulating`
  (if (== (`KismetMathLibrary.VSize` (`SceneComponent.GetComponentVelocity` (`self.Vent`))) 0.0)
    (`PrimitiveComponent.SetSimulatePhysics` (`self.Vent`) false)
    (`KismetSystemLibrary.K2_ClearAndInvalidateTimerHandle` (`self.SimTimer`))
    (`ActorComponent.K2_DestroyComponent` (`self.VentilationParticles`))))

(fn `UserConstructionScript`)