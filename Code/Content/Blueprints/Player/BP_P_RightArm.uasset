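; Right arm player Blueprint whose throw input, while aiming and off cooldown, pulls the targeted pushable object or body part toward itself.
; ActivatePull enables cone collisions and queries the aimed actor, then applies an impulse to pushables or a scaled launch to body parts, using Metrics strengths.
; A successful pull stops the target's geyser animation, flags the cooldown and disables the cones; an invalid target only plays failure feedback.
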(event `EnhancedInput|/Game/Input/Actions/IA_Throw`
  (params (ActionValue :type Boolean) (ElapsedSeconds :type "Float (double-precision)") (TriggeredSeconds :type "Float (double-precision)") (InputAction :type "InputAction Object Reference" :default "/Game/Input/Actions/IA_Throw.IA_Throw"))
  (:`Triggered`
    (if (`self.aiming`)
      (if (not (`self.powerInCooldown`))
        (`self.ActivatePull`)
        (`self.RechargeCooldown`)))))

(fn `ActivatePull`
  (`PrimitiveComponent.SetCollisionEnabled` (`self.CollisionCone`) "QueryAndPhysics")
  (`PrimitiveComponent.SetCollisionEnabled` (`self.AimingCone`) "QueryAndPhysics")
  (bind (_isvalid _actoraffected) (`self.aimingCollision`))
  (if _isvalid
    (`self.PlaySFX` "NewEnumerator0")
    (`KismetSystemLibrary.PrintText` "Pull")
    (bind _asbp_a_pushable (cast `/Game/Blueprints/Interactive/Physical/BP_A_Pushable` _actoraffected)
      (:`then`
        (`/Game/Blueprints/Interactive/Physical/BP_A_Pushable.StopAnim_Geyser` _asbp_a_pushable)
        (`PrimitiveComponent.AddImpulse` (`/Game/Blueprints/Interactive/Physical/BP_A_Pushable.BoxSkin` _asbp_a_pushable) (* (`KismetMathLibrary.GetDirectionUnitVector` (`self.K2_GetActorLocation` _asbp_a_pushable) (`self.K2_GetActorLocation`)) (`.PullPowerObject_32_BBFBF53947B8372A0E2F0E947BD79DB6` (break `/Game/Blueprints/Player/Metrics/Metrics_Arm` (`self.metrics`)))) "None" false))
      (:`CastFailed`
        (bind _asbpp_body_part (cast `/Game/Blueprints/Player/BPP_BodyPart` _actoraffected))
        (`self.StopAnim_Geyser` _asbpp_body_part)
        (`self.LaunchCharacter` _asbpp_body_part (/ (* (`KismetMathLibrary.GetDirectionUnitVector` (`self.K2_GetActorLocation` _asbpp_body_part) (`self.K2_GetActorLocation`)) (`.PullPowerBodyPart_34_3C79843D4D3CCFC7706AED9FC03416DB` (break `/Game/Blueprints/Player/Metrics/Metrics_Arm` (`self.metrics`)))) 100.0) false false)))
    (set `self.powerInCooldown` true)
    (`PrimitiveComponent.SetCollisionEnabled` (`self.CollisionCone`) "NoCollision")
    (`PrimitiveComponent.SetCollisionEnabled` (`self.AimingCone`) "NoCollision")
    (else
      (`self.PlaySFX` "NewEnumerator12")
      (`KismetSystemLibrary.PrintText` "Impossible de pull"))))

(fn `UserConstructionScript`
  (`parent.UserConstructionScript`))