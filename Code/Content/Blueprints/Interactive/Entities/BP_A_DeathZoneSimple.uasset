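; Death zone actor that sends body parts and pushable objects back to their respawn state when they overlap it.
; Every overlap first plays an interactive sound through the cached game instance.
; An arm first runs RespawnThrow and continues to the normal respawn only if that returns true.
; Body parts call their own Respawn, while pushables return to their initial transform with linear velocity zeroed.
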(event `self.ReceiveBeginPlay`
  (`self.InitGameInstance`))

(event `self.ReceiveActorBeginOverlap`
  (params (OtherActor :type "Actor Object Reference"))
  (`self.PlaySFX` "NewEnumerator17")
  (bind _asbpp_p_arm (cast `/Game/Blueprints/Player/BPP_P_Arm` OtherActor)
    (:`then`
      (bind _defaultbehavior (`/Game/Blueprints/Player/BPP_P_Arm.RespawnThrow` _asbpp_p_arm))
      (if _defaultbehavior
        (bind _asbpp_body_part (cast `/Game/Blueprints/Player/BPP_BodyPart` OtherActor :!label _label)
          (:`then`
            (`/Game/Blueprints/Player/BPP_BodyPart.Respawn` _asbpp_body_part))
          (:`CastFailed`
            ;[0.02016 0.041 0.15 0.5 40] Reset actor transform and physics to initial transform
            (bind _asbp_a_pushable (cast `/Game/Blueprints/Interactive/Physical/BP_A_Pushable` OtherActor))
            (`self.K2_SetActorTransform` _asbp_a_pushable (`/Game/Blueprints/Interactive/Physical/BP_A_Pushable.InitialTransform` _asbp_a_pushable) false false)
            (`PrimitiveComponent.SetPhysicsLinearVelocity` (`/Game/Blueprints/Interactive/Physical/BP_A_Pushable.BoxSkin` _asbp_a_pushable) (0.0 0.0 0.0) false "None")))))
    (:`CastFailed`
      (goto _label))))

(fn `InitGameInstance`
  (bind _asbp_gi_ew_game_instance (cast `/Game/Blueprints/Managing/BP_GI_EwGameInstance` (`GameplayStatics.GetGameInstance`)))
  (set `self.GameInstance` _asbp_gi_ew_game_instance))

(fn `PlaySFX`
  (params (Type :type "/Game/Utilities/ESFX_Enviro Enum" :default "NewEnumerator0"))
  (`/Game/Blueprints/Managing/BP_GI_EwGameInstance.PlayInteractiveSound` (`self.GameInstance`) self Type))

(fn `UserConstructionScript`)