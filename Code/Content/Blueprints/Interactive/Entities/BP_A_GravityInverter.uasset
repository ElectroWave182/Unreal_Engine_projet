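; Overlap-triggered gravity inverter that sets player body parts and pushable boxes to inverted or normal gravity, depending on its Inverse flag.
; Body parts get a new gravity direction, inverted camera controls and updated respawn data, while Tick animates their camera roll through a map of pending rotations.
; Boxes toggle physics gravity, flip with a scale-based height offset and reset their velocity and initial position.
; Each overlap plays a direction-specific sound via the GameInstance.
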(event `self.ReceiveActorBeginOverlap`
  (params (OtherActor :type "Actor Object Reference"))
  (`self.PlaySFX`)
  (`self.inverserGravite` OtherActor))

(event `self.ReceiveTick`
  (params (DeltaSeconds :type "Float (single-precision)"))
  (`self.animer` DeltaSeconds))

(event `self.ReceiveBeginPlay`
  (bind _asbp_gi_ew_game_instance (cast `/Game/Blueprints/Managing/BP_GI_EwGameInstance` (`GameplayStatics.GetGameInstance`)))
  (set `self.GameInstance` _asbp_gi_ew_game_instance))

(fn `animer`
  (params (dureeImage :type "Float (double-precision)"))
  ;[0.7344 0.7344 0.7344 0.5] Parcours des objets à animer
  (bind _keys (`BlueprintMapLibrary.Map_Keys` (`self.aAnimer`)))
  (for _array_element _keys
    (bind _value (`BlueprintMapLibrary.Map_Find` (`self.aAnimer`) _array_element))
    ;[0.7344 0.7344 0.7344 0.5] Animation de la rotation de caméra
    (`self.animerCamera` _array_element (`KismetMathLibrary.BreakVector2D` _value) (`.Y` (`KismetMathLibrary.BreakVector2D` _value)) (`local.dureeImage`))))

(fn `animerCamera`
  (params (personnage :type "/Game/Blueprints/Player/BPP_BodyPart Object Reference") (angleActuel :type "Float (double-precision)") (angleFinal :type "Float (double-precision)") (dureeImage :type "Float (double-precision)"))
  (locals (sens :type "Float (double-precision)") (camera :type "CameraComponent Object Reference"))
  (bind _personnage (`local.personnage`))
  (bind _dureeimage (`local.dureeImage`))
  (bind _angleactuel (`local.angleActuel`))
  (bind (_returnvalue_roll _returnvalue_pitch _returnvalue_yaw) (`KismetMathLibrary.BreakRotator` (`SceneComponent.K2_GetComponentRotation` (`/Game/Blueprints/Player/BPP_BodyPart.FollowCamera` personnage))))
  (bind _followcamera (`/Game/Blueprints/Player/BPP_BodyPart.FollowCamera` _personnage))
  (bind (_returnvalue_roll_2 _returnvalue_pitch_2 _returnvalue_yaw_2) (`KismetMathLibrary.BreakRotator` (`SceneComponent.K2_GetComponentRotation` _followcamera)))
  (bind _returnvalue (+ (/ (* _dureeimage (`local.sens`) 180.0) (`self.dureeAnimation`)) _angleactuel))
  ;[0.7448 0.7448 0.7448 0.5] Paramètres
  (set `local.camera` (`/Game/Blueprints/Player/BP_P_Torso.FollowCamera` personnage))
  (bind _sens (`self.sensRotation` (`local.angleFinal`) _angleactuel))
  (set `local.sens` _sens)
  (bind _arret (`self.conditionArret` (`local.angleFinal`) _angleactuel _dureeimage))
  (if _arret
    ;[0.7917 0.7917 0.7917 0.5] La rotation est terminée, on la passe à l'objectif et on la retire du dictionnaire à animer
    (`BlueprintMapLibrary.Map_Remove` (`self.aAnimer`) _personnage)
    (`SceneComponent.K2_SetWorldRotation` _followcamera (`KismetMathLibrary.MakeRotator` (`local.angleFinal`) _returnvalue_pitch_2 _returnvalue_yaw_2) false false)
    (else
      ;[0.7656 0.7656 0.7656 0.5] La rotation se poursuit et on la stocke
      (`/Game/Utilities/BP_Dictionnaire.associer` (`self.aAnimer`) (`local.personnage`) (`KismetMathLibrary.MakeVector2D` _returnvalue (`local.angleFinal`)))
      (`SceneComponent.K2_SetWorldRotation` (`/Game/Blueprints/Player/BPP_BodyPart.FollowCamera` (`local.personnage`)) (`KismetMathLibrary.MakeRotator` _returnvalue _returnvalue_pitch _returnvalue_yaw) false false))))

(fn `conditionArret`
  (params (objectif :type "Float (double-precision)") (actuelle :type "Float (double-precision)") (periode :type "Float (double-precision)"))
  (returns (arret :type Boolean))
  (return (< (`KismetMathLibrary.Abs` (- objectif actuelle)) (* periode 180.0))))

(fn `inverserGravite`
  (params (objet :type "Actor Object Reference"))
  (locals (personnage :type "/Game/Blueprints/Player/BPP_BodyPart Object Reference"))
  (bind _returnvalue (`KismetMathLibrary.MakeVector` 0.0 0.0 -1.0))
  (bind _returnvalue_2 (`KismetMathLibrary.MakeVector` 0.0 0.0 1.0))
  (bind _cameraangle (`self.CameraAngle`))
  (bind _inverse (`self.Inverse`))
  (bind _charactermovement (`Character.CharacterMovement` (`local.personnage`)))
  (bind _gravitydirection (`CharacterMovementComponent.GravityDirection` _charactermovement))
  ;[0.8021 0.8021 0.8021 0.5] Paramètres
  (bind _asbpp_body_part (cast `/Game/Blueprints/Player/BPP_BodyPart` objet)
    (:`then`
      (bind _output_get (set `local.personnage` _asbpp_body_part))
      (if _inverse
        (if (!= _returnvalue_2 _gravitydirection :`ErrorTolerance` 0.1)
          (`CharacterMovementComponent.SetGravityDirection` _charactermovement _returnvalue_2)
          (set `self.CameraAngle` 180.0)
          ;[0.7812 0.7812 0.7812 0.5] Inverse les contrôles du joueur pour qu'ils soient cohérents avec la caméra
          (`/Game/Blueprints/Player/BP_P_Torso.inverserCamera` _output_get :!label _label)
          (`/Game/Blueprints/Player/BPP_BodyPart.SetRespawnDataToCurrent` _output_get)
          ;[0.776 0.776 0.776 0.5] Ajoute le personnage dans le dictionnaire des objets à animer
          (`/Game/Utilities/BP_Dictionnaire.associer` (`self.aAnimer`) (`local.personnage`) (`KismetMathLibrary.MakeVector2D` (- 180.0 _cameraangle) _cameraangle))
          (bind _asbp_p_torso (cast `/Game/Blueprints/Player/BP_P_Torso` (`local.personnage`)))
          (set `/Game/Blueprints/Player/BP_P_Torso.IsAffectedByGravityInverter` true _asbp_p_torso)
          (set `/Game/Blueprints/Player/BP_P_Torso.GravityInverter` self _asbp_p_torso))
        (elif (!= _gravitydirection _returnvalue :`ErrorTolerance` 0.1)
          (`CharacterMovementComponent.SetGravityDirection` _charactermovement _returnvalue)
          (set `self.CameraAngle` 0.0)
          (goto _label))))
    (:`CastFailed`
      ; Inversion de la caisse
      (bind _asbp_a_pushable (cast `/Game/Blueprints/Interactive/Physical/BP_A_Pushable` objet))
      (if _inverse
        (bind _isinversed (`/Game/Blueprints/Interactive/Physical/BP_A_Pushable.isInversed` _asbp_a_pushable))
        (if (not _isinversed)
          (set `/Game/Blueprints/Interactive/Physical/BP_A_Pushable.isInversed` true _asbp_a_pushable)
          (bind _boxskin (`/Game/Blueprints/Interactive/Physical/BP_A_Pushable.BoxSkin` _asbp_a_pushable))
          (`PrimitiveComponent.SetEnableGravity` _boxskin false)
          (`PrimitiveComponent.SetConstraintMode` _boxskin "None")
          (`self.K2_SetActorRotation` _asbp_a_pushable (struct :`Roll` 180.0) false)
          (bind _returnvalue_3 (`self.K2_GetActorLocation` _asbp_a_pushable))
          (bind (_returnvalue_x _returnvalue_y _returnvalue_z) (`KismetMathLibrary.BreakVector` (`self.GetActorScale3D` _asbp_a_pushable)))
          (bind _returnvalue_4 (`KismetMathLibrary.MakeVector` 0.0 0.0 (* _returnvalue_z 92.5)))
          (`self.K2_SetActorLocation` _asbp_a_pushable (+ _returnvalue_3 _returnvalue_4) false false)
          (`PrimitiveComponent.SetConstraintMode` _boxskin "Default")
          (set `/Game/Blueprints/Interactive/Physical/BP_A_Pushable.InitPosition` (`self.K2_GetActorLocation` _asbp_a_pushable) _asbp_a_pushable :!label _label_2)
          (`PrimitiveComponent.SetPhysicsLinearVelocity` _boxskin (0.0 0.0 0.0) false "None"))
        (elif _isinversed
          (set `/Game/Blueprints/Interactive/Physical/BP_A_Pushable.isInversed` false _asbp_a_pushable)
          (`PrimitiveComponent.SetEnableGravity` _boxskin true)
          (`PrimitiveComponent.SetConstraintMode` _boxskin "None")
          (`self.K2_SetActorRotation` :`self` _asbp_a_pushable)
          (`self.K2_SetActorLocation` _asbp_a_pushable (- _returnvalue_3 _returnvalue_4) false false)
          (`PrimitiveComponent.SetConstraintMode` _boxskin "Default")
          (goto _label_2))))))

(fn `PlaySFX`
  (bind _gameinstance (`self.GameInstance`))
  (bind _gameinstance_2 (`self.GameInstance`))
  (if (`self.Inverse`)
    (`/Engine/EditorBlueprintResources/StandardMacros.IsValid` _gameinstance_2
      (:`Is Valid`
        (`/Game/Blueprints/Managing/BP_GI_EwGameInstance.PlayInteractiveSound` _gameinstance_2 self "NewEnumerator8")))
    (else
      (`/Engine/EditorBlueprintResources/StandardMacros.IsValid` _gameinstance
        (:`Is Valid`
          (`/Game/Blueprints/Managing/BP_GI_EwGameInstance.PlayInteractiveSound` _gameinstance self "NewEnumerator9"))))))

(fn `sensRotation`
  (params (objectif :type "Float (double-precision)") (actuel :type "Float (double-precision)"))
  (returns (sens :type "Float (double-precision)"))
  (return (`KismetMathLibrary.SignOfFloat` (- objectif actuel))))

(fn `UserConstructionScript`)