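; Lounge eye actor that rotates to look at the player, either constantly or only while body parts are inside its Collisionbox.
; With AlwaysLooking set, Tick turns it toward player character 0; otherwise it faces the tracked BPP_BodyPart while WillLook is set.
; Overlap begin targets the newest body part; overlap end falls back to another overlapping part or stops tracking.
; The construction script's sphere radius setter is disconnected.
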(event `self.ReceiveTick`
  (params (DeltaSeconds :type "Float (single-precision)"))
  (bind _returnvalue (`self.K2_GetActorLocation`))
  (bind _returnvalue_2 (`GameplayStatics.GetPlayerCharacter` 0))
  (if (`self.alwaysLooking`)
    (`/Engine/EditorBlueprintResources/StandardMacros.IsValid` _returnvalue_2
      (:`Is Valid`
        (`self.K2_SetActorRotation` (`KismetMathLibrary.FindLookAtRotation` _returnvalue (`self.K2_GetActorLocation` _returnvalue_2)))))
    (elif (`self.willLook`)
      (`self.K2_SetActorRotation` (`KismetMathLibrary.FindLookAtRotation` _returnvalue (`self.K2_GetActorLocation` (`self.playerRef`)))))))

(event `self.Collisionbox.OnActorBeginOverlap`
  (params (OverlappedActor :type "Actor Object Reference") (OtherActor :type "Actor Object Reference"))
  (bind _asbpp_body_part (cast `/Game/Blueprints/Player/BPP_BodyPart` OtherActor))
  (set `self.willLook` true)
  (set `self.playerRef` _asbpp_body_part))

(event `self.Collisionbox.OnActorEndOverlap`
  (params (OverlappedActor :type "Actor Object Reference") (OtherActor :type "Actor Object Reference"))
  (bind _allbodyparts (`self.allBodyParts`))
  (if (`KismetMathLibrary.ClassIsChildOf` (`GameplayStatics.GetObjectClass` OtherActor) "/Game/Blueprints/Player/BPP_BodyPart.BPP_BodyPart_C")
    (set `self.allBodyParts` (`PrimitiveComponent.GetOverlappingActors` (`TriggerBase.SpriteComponent` (`self.Collisionbox`)) "/Game/Blueprints/Player/BPP_BodyPart.BPP_BodyPart_C"))
    (if (== (`KismetArrayLibrary.Array_Length` _allbodyparts) 0)
      (set `self.willLook` false)
      (elif (not (`KismetArrayLibrary.Array_Contains` _allbodyparts (`self.playerRef`)))
        (set `self.playerRef` (cast `/Game/Blueprints/Player/BPP_BodyPart` (`|GetArrayItem` _allbodyparts) :!pure true))))))

(fn `UserConstructionScript`)