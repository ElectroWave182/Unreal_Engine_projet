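; Mirror character actor that copies the look of a referenced character onto its own skeletal mesh.
; Each tick it matches the relative scale of the referenced character's mesh.
; If the character is a BP_P_Torso, it also copies every material slot by index to keep hidden body parts in sync.
; The actor destroys itself once the character reference is invalid.
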(event `self.ReceiveTick`
  (params (DeltaSeconds :type "Float (single-precision)"))
  (bind _characterref (`self.CharacterRef`))
  (`/Engine/EditorBlueprintResources/StandardMacros.IsValid` _characterref
    (:`Is Valid`
      (`SceneComponent.SetRelativeScale3D` (`self.SkeletalMesh`) (`SceneComponent.RelativeScale3D` (`Character.Mesh` _characterref)))
      ; Update hide bodyparts
      (bind _asbp_p_torso (cast `/Game/Blueprints/Player/BP_P_Torso` (`self.CharacterRef`)))
      (for (_array_element _array_index) (`MeshComponent.GetMaterials` (`Character.Mesh` _asbp_p_torso))
        (`PrimitiveComponent.SetMaterial` (`self.SkeletalMesh`) _array_index _array_element)))
    (:`Is Not Valid`
      (`self.K2_DestroyActor`))))

(fn `UserConstructionScript`)