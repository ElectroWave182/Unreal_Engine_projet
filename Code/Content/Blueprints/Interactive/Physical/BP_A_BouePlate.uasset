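; Interactive platform that a BPP_P_Leg can pass through by stomping from above or charge-jumping from below, relative to its gravity.
; Upper and lower trigger boxes start the pass, tracking one leg, ignoring capsule Destructible and mesh Camera collision, and playing a sound.
; Leaving the opposite box restores collision and clears the stomp.
; Mesh hits from the torso or a leg spawn a contact cloud effect.
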(event `self.LowerBox.OnComponentBeginOverlap`
  (params (OverlappedComponent :type "PrimitiveComponent Object Reference") (OtherActor :type "Actor Object Reference") (OtherComp :type "PrimitiveComponent Object Reference") (OtherBodyIndex :type Integer) (bFromSweep :type Boolean) (SweepResult :type "HitResult Structure (by ref)"))
  ; When BPP_P_Leg is stomping from under
  (bind _asbpp_p_leg (cast `/Game/Blueprints/Player/BPP_P_Leg` OtherActor))
  (bind (_gravitydirection_x _gravitydirection_y _gravitydirection_z) (`KismetMathLibrary.BreakVector` (`CharacterMovementComponent.GravityDirection` (`Character.CharacterMovement` _asbpp_p_leg))))
  (if (< _gravitydirection_z 0.0)
    (`self.ChargedJumpEnter` _asbpp_p_leg)
    (else
      (`self.StompEnter` _asbpp_p_leg))))

(event `self.LowerBox.OnComponentEndOverlap`
  (params (OverlappedComponent :type "PrimitiveComponent Object Reference") (OtherActor :type "Actor Object Reference") (OtherComp :type "PrimitiveComponent Object Reference") (OtherBodyIndex :type Integer))
  ; When BPP_P_Leg is stomping from upper and pass through
  (bind _asbpp_p_leg (cast `/Game/Blueprints/Player/BPP_P_Leg` OtherActor))
  (`self.StompExit` OverlappedComponent _asbpp_p_leg))

(event `ChargedJumpEnter`
  (params (Leg :type "/Game/Blueprints/Player/BPP_P_Leg Object Reference"))
  ; Leg charged jump
  (if (and (`/Game/Blueprints/Player/BPP_P_Leg.IsChargedJump` Leg) (== (`self.LegToKeepTrack`) null))
    (set `self.LegToKeepTrack` Leg)
    (set `self.BoueCollider` (`self.UpperBox`))
    (`PrimitiveComponent.SetCollisionResponseToChannel` (`Character.CapsuleComponent` Leg) "ECC_Destructible" "ECR_Ignore")
    (`PrimitiveComponent.SetCollisionResponseToChannel` (`self.Mesh`) "ECC_Camera" "ECR_Ignore" :!label _label)
    (`self.PlaySFX` "NewEnumerator14")))

(event `self.UpperBox.OnComponentBeginOverlap`
  (params (OverlappedComponent :type "PrimitiveComponent Object Reference") (OtherActor :type "Actor Object Reference") (OtherComp :type "PrimitiveComponent Object Reference") (OtherBodyIndex :type Integer) (bFromSweep :type Boolean) (SweepResult :type "HitResult Structure (by ref)"))
  ; When BPP_P_Leg is stomping from upper
  (bind _asbpp_p_leg (cast `/Game/Blueprints/Player/BPP_P_Leg` OtherActor))
  (bind (_gravitydirection_x _gravitydirection_y _gravitydirection_z) (`KismetMathLibrary.BreakVector` (`CharacterMovementComponent.GravityDirection` (`Character.CharacterMovement` _asbpp_p_leg))))
  (if (< _gravitydirection_z 0.0)
    (`self.StompEnter` _asbpp_p_leg)
    (else
      (`self.ChargedJumpEnter` _asbpp_p_leg))))

(event `StompEnter`
  (params (Leg :type "/Game/Blueprints/Player/BPP_P_Leg Object Reference"))
  ; Leg stomp
  (if (and (`/Game/Blueprints/Player/BPP_P_Leg.IsStomping` Leg) (== (`self.LegToKeepTrack`) null))
    (set `self.LegToKeepTrack` Leg)
    (set `self.BoueCollider` (`self.LowerBox`))
    (`PrimitiveComponent.SetCollisionResponseToChannel` (`Character.CapsuleComponent` Leg) "ECC_Destructible" "ECR_Ignore")
    (goto _label)))

(event `self.UpperBox.OnComponentEndOverlap`
  (params (OverlappedComponent :type "PrimitiveComponent Object Reference") (OtherActor :type "Actor Object Reference") (OtherComp :type "PrimitiveComponent Object Reference") (OtherBodyIndex :type Integer))
  ; When BPP_P_Leg is stomping from under and pass through
  (bind _asbpp_p_leg (cast `/Game/Blueprints/Player/BPP_P_Leg` OtherActor))
  (`self.StompExit` OverlappedComponent _asbpp_p_leg))

(event `StompExit`
  (params (OverlappedComponent :type "PrimitiveComponent Object Reference") (Leg :type "/Game/Blueprints/Player/BPP_P_Leg Object Reference"))
  (bind _legtokeeptrack (`self.LegToKeepTrack`))
  ; Leg exits platform
  (if (and (== OverlappedComponent (`self.BoueCollider`)) (== Leg _legtokeeptrack))
    (set `/Game/Blueprints/Player/BPP_P_Leg.IsStomping` false Leg)
    (`PrimitiveComponent.SetCollisionResponseToChannel` (`Character.CapsuleComponent` _legtokeeptrack) "ECC_Destructible" "ECR_Block")
    (set `self.LegToKeepTrack` null)
    (set `self.BoueCollider` null)
    (`PrimitiveComponent.SetCollisionResponseToChannel` (`self.Mesh`) "ECC_Camera" "ECR_Block")))

(event `self.Mesh.OnComponentHit`
  (params (HitComponent :type "PrimitiveComponent Object Reference") (OtherActor :type "Actor Object Reference") (OtherComp :type "PrimitiveComponent Object Reference") (NormalImpulse :type "Vector Structure") (Hit :type "HitResult Structure (by ref)"))
  (bind _asbp_p_torso (cast `/Game/Blueprints/Player/BP_P_Torso` OtherActor)
    (:`then`
      (bind _returnvalue (`self.K2_GetActorLocation` _asbp_p_torso))
      (`NiagaraFunctionLibrary.SpawnSystemAtLocation` "/Game/Assets/VFX/NS_ContactNuage.NS_ContactNuage" (+ _returnvalue (0.0 0.0 -50.0))))
    (:`CastFailed`
      (bind _asbpp_p_leg (cast `/Game/Blueprints/Player/BPP_P_Leg` OtherActor))
      (bind _returnvalue_2 (`self.K2_GetActorLocation` _asbpp_p_leg))
      (`NiagaraFunctionLibrary.SpawnSystemAtLocation` "/Game/Assets/VFX/NS_ContactNuage.NS_ContactNuage" (+ _returnvalue_2 (0.0 0.0 -40.0))))))

(fn `isWeightSuffisient`
  (params (Object :type "Object Object Reference"))
  (returns (ReturnValue :type Boolean))
  (return false))

(fn `UserConstructionScript`)