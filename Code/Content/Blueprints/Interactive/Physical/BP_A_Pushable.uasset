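; Pushable physics crate that body-part pawns can move when they meet its required-part conditions.
; Side overlap volumes check those conditions, then unblock the NotPush collider, flag pushing, switch the HUD and play push audio.
; Tick ground-traces to update position or fade the sound, and applies upward force when gravity is inverted.
; Geyser timelines lift and center the box, DeathBox respawns body parts it hits, and construction sets its color material.
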(event `self.ReceiveTick`
  (params (DeltaSeconds :type "Float (single-precision)"))
  (bind _boxskin (`self.BoxSkin`))
  ; Set the position before falling
  (bind _isgrounded (`self.CheckGround`))
  (if (and _isgrounded (`self.isMoving`))
    (set `self.InitPosition` (`self.K2_GetActorLocation`))
    (else
      (`self.StopPushSFX`)))
  ; Apply inversed gravity
  (if (`self.isInversed`)
    (`PrimitiveComponent.AddForce` _boxskin (* (`PrimitiveComponent.GetMass` _boxskin) (0.0 0.0 980.0)) "None" false)))

(event `StartHover`
  ;[0.15 0.07344 0.07344 0.5 50] Overlay
  (`MeshComponent.SetOverlayMaterial` (`self.BoxSkin`) "/Game/Assets/Materials/M_OverlayPushPull.M_OverlayPushPull"))

(event `self.ReceiveBeginPlay`
  ; Initialize the mass and position
  (`self.InitGameInstance`)
  (`PrimitiveComponent.SetMassOverrideInKg` (`self.BoxSkin`) "None" (`self.Mass in Kg`) true)
  (set `self.InitPosition` (`self.K2_GetActorLocation`))
  ;; Najib : For Respawn
  (set `self.InitialTransform` (`self.GetTransform`)))

(event `EndHover`
  ;[0.15 0.07344 0.07344 0.5 50] Overlay
  (`MeshComponent.SetOverlayMaterial` (`self.BoxSkin`) null))

(event `self.CollisionX.OnComponentBeginOverlap`
  (params (OverlappedComponent :type "PrimitiveComponent Object Reference") (OtherActor :type "Actor Object Reference") (OtherComp :type "PrimitiveComponent Object Reference") (OtherBodyIndex :type Integer) (bFromSweep :type Boolean) (SweepResult :type "HitResult Structure (by ref)"))
  ; Enable the movement
  (bind _canpush (`self.ActivatePushing`))
  (if _canpush
    (bind _asbpp_body_part (cast `/Game/Blueprints/Player/BPP_BodyPart` OtherActor))
    (set `/Game/Blueprints/Player/BPP_BodyPart.IsPushing?` true _asbpp_body_part)
    (bind _asbp_gi_ew_game_instance (cast `/Game/Blueprints/Managing/BP_GI_EwGameInstance` (`GameplayStatics.GetGameInstance`) :!label _label))
    (`/Game/Blueprints/Managing/BP_GI_EwGameInstance.ToggleHudInGameInstance` _asbp_gi_ew_game_instance "NewEnumerator5" null null)))

(event `self.CollisionY.OnComponentBeginOverlap`
  (params (OverlappedComponent :type "PrimitiveComponent Object Reference") (OtherActor :type "Actor Object Reference") (OtherComp :type "PrimitiveComponent Object Reference") (OtherBodyIndex :type Integer) (bFromSweep :type Boolean) (SweepResult :type "HitResult Structure (by ref)"))
  ; Enable the movement
  (bind _canpush (`self.ActivatePushing`))
  (if _canpush
    (bind _asbpp_body_part (cast `/Game/Blueprints/Player/BPP_BodyPart` OtherActor))
    (set `/Game/Blueprints/Player/BPP_BodyPart.IsPushing?` true _asbpp_body_part)
    (goto _label)))

(event `self.CollisionY.OnComponentEndOverlap`
  (params (OverlappedComponent :type "PrimitiveComponent Object Reference") (OtherActor :type "Actor Object Reference") (OtherComp :type "PrimitiveComponent Object Reference") (OtherBodyIndex :type Integer))
  ; Disable the movement
  (bind _asbpp_body_part (cast `/Game/Blueprints/Player/BPP_BodyPart` OtherActor))
  (set `/Game/Blueprints/Player/BPP_BodyPart.IsPushing?` false _asbpp_body_part)
  (`PrimitiveComponent.SetCollisionResponseToChannel` (`self.NotPush`) "ECC_Pawn" "ECR_Block" :!label _label_2)
  (set `self.isMoving` false)
  (bind _asbp_gi_ew_game_instance (cast `/Game/Blueprints/Managing/BP_GI_EwGameInstance` (`GameplayStatics.GetGameInstance`)))
  (if (`|EnumEquality` (`/Game/Blueprints/Managing/BP_GI_EwGameInstance.ECurrentHud` _asbp_gi_ew_game_instance) "NewEnumerator5")
    (`/Game/Blueprints/Managing/BP_GI_EwGameInstance.ToggleHudInGameInstance` _asbp_gi_ew_game_instance (`/Game/Blueprints/Managing/BP_GI_EwGameInstance.EOldHud` _asbp_gi_ew_game_instance) null null)))

(event `self.CollisionX.OnComponentEndOverlap`
  (params (OverlappedComponent :type "PrimitiveComponent Object Reference") (OtherActor :type "Actor Object Reference") (OtherComp :type "PrimitiveComponent Object Reference") (OtherBodyIndex :type Integer))
  ; Disable the movement
  (bind _asbpp_body_part (cast `/Game/Blueprints/Player/BPP_BodyPart` OtherActor))
  (set `/Game/Blueprints/Player/BPP_BodyPart.IsPushing?` false _asbpp_body_part)
  (goto _label_2))

(event `RecheckBodyPart`
  (bind _notpush (`self.NotPush`))
  ; Recheck the bodyparts
  (bind _isvalid (`self.CheckPawnConditions`))
  (if _isvalid
    (`PrimitiveComponent.SetCollisionResponseToChannel` _notpush "ECC_Pawn" "ECR_Ignore")
    (else
      (`PrimitiveComponent.SetCollisionResponseToChannel` _notpush "ECC_Pawn" "ECR_Block"))))

(event `PlayAnim_Geyser`
  (bind _maxheight (`self.MaxHeight`))
  (bind _elevatorz (`self.elevatorZ`))
  (bind (_initgeyserlocation_x _initgeyserlocation_y) (`KismetMathLibrary.BreakVector` (`self.InitGeyserLocation`)))
  (bind (_initgeyserlocation_x_2 _initgeyserlocation_y_2 _initgeyserlocation_z) (`KismetMathLibrary.BreakVector` (`self.InitGeyserLocation`)))
  (bind _boxskin (`self.BoxSkin`))
  ; Geyser animation
  (bind (_direction _geyservelocity) (`Timeline|geyserEnCours` :`NewTime` (/ (- _initgeyserlocation_z _elevatorz) _maxheight) :!label _label_3)
    (:`Update`
      (`PrimitiveComponent.SetPhysicsLinearVelocity` _boxskin (0.0 0.0 0.0) false "None")
      (bind (_returnvalue_x _returnvalue_y _returnvalue_z) (`KismetMathLibrary.BreakVector` (`self.K2_GetActorLocation` (stale `InitAnim_Geyser` _output_get))))
      (bind (_returnvalue_x_2 _returnvalue_y_2) (`KismetMathLibrary.BreakVector` (`KismetMathLibrary.VLerp` (`KismetMathLibrary.MakeVector` _initgeyserlocation_x _initgeyserlocation_y) (`KismetMathLibrary.MakeVector` _returnvalue_x _returnvalue_y) (stale `InitAnim_Geyser` _alphatocenter))))
      (`KismetSystemLibrary.MoveComponentTo` _boxskin (- (`KismetMathLibrary.MakeVector` _returnvalue_x_2 _returnvalue_y_2 (+ (* _geyservelocity _maxheight) _elevatorz)) (`self.InitLocation`)) (`SceneComponent.RelativeRotation` _boxskin) false false 0.001 :!label _label_4))))

(event `StopAnim_Geyser`
  ; Geyser animation
  (goto _label_3 :!via `Stop`))

(event `InitAnim_Geyser`
  (params (Geyser :type "/Game/Blueprints/Interactive/Receiver/BP_A_Elevator Object Reference") (MaxHeight :type "Float (double-precision)"))
  (bind _boxskin (`self.BoxSkin`))
  ; Geyser animation
  (bind _output_get (set `self.elevator` Geyser))
  (set `self.InitGeyserLocation` (`SceneComponent.K2_GetComponentLocation` _boxskin))
  (`PrimitiveComponent.SetEnableGravity` _boxskin false)
  (bind (_returnvalue_x _returnvalue_y _returnvalue_z) (`KismetMathLibrary.BreakVector` (`self.K2_GetActorLocation` _output_get)))
  (set `self.elevatorZ` _returnvalue_z)
  (set `self.MaxHeight` MaxHeight)
  (`|ExecutionSequence`
    (:`then_0`
      (goto _label_3 :!via `SetNewTime`))
    (:`then_1`
      (bind (_direction _alphatocenter) (`Timeline|CenterTheBox` :!via `SetNewTime` :!label _label_5)
        (:`Update`
          (goto _label_4))))
    (:`then_2`
      (goto _label_5))))

(event `self.DeathBox.OnComponentBeginOverlap`
  (params (OverlappedComponent :type "PrimitiveComponent Object Reference") (OtherActor :type "Actor Object Reference") (OtherComp :type "PrimitiveComponent Object Reference") (OtherBodyIndex :type Integer) (bFromSweep :type Boolean) (SweepResult :type "HitResult Structure (by ref)"))
  ; Kill the bodypart if the pushable fall on it
  (bind _asbpp_body_part (cast `/Game/Blueprints/Player/BPP_BodyPart` OtherActor))
  (`/Game/Blueprints/Player/BPP_BodyPart.Respawn` _asbpp_body_part))

(fn `ActivatePushing`
  (returns (canPush :type Boolean))
  (if (`PrimitiveComponent.IsGravityEnabled` (`self.BoxSkin`))
    (bind _isvalid (`self.CheckPawnConditions`))
    (if _isvalid
      (`PrimitiveComponent.SetCollisionResponseToChannel` (`self.NotPush`) "ECC_Pawn" "ECR_Ignore")
      (set `self.isMoving` true)
      (`self.PlayPushSFX`))
    (return _isvalid)))

(fn `ApplyMaterialColor`
  (`PrimitiveComponent.SetMaterial` (`self.BoxSkin`) 0 (`self.Material to Apply`)))

(fn `CheckGround`
  (returns (isGrounded :type Boolean))
  (locals (CheckVector :type "Vector Structure"))
  (bind _returnvalue (`self.K2_GetActorLocation`))
  (if (`self.isInversed`)
    (set `local.CheckVector` (0.0 0.0 10.0))
    (else
      (set `local.CheckVector` (0.0 0.0 -10.0))))
  (bind (_outhit _returnvalue_2) (`KismetSystemLibrary.LineTraceSingle` _returnvalue (+ _returnvalue (`local.CheckVector`)) "TraceTypeQuery2"))
  (return _returnvalue_2))

(fn `CheckPawnConditions`
  (returns (IsValid :type Boolean))
  (bind _pawnconditions (`self.pawnConditions`))
  (bind _value (`BlueprintMapLibrary.Map_Find` _pawnconditions "2 Jambes"))
  (bind _value_2 (`BlueprintMapLibrary.Map_Find` _pawnconditions "1 Jambe"))
  (bind _value_3 (`BlueprintMapLibrary.Map_Find` _pawnconditions "2 Bras"))
  (bind _value_4 (`BlueprintMapLibrary.Map_Find` _pawnconditions "Torse"))
  (bind _value_5 (`BlueprintMapLibrary.Map_Find` _pawnconditions "1 Bras"))
  ; Checks if the current pawn contains all of the required parts, still returns true if it has more parts than required
  ; Example : [1,1,1,0,1,0] means [torso, head, one arm, one leg]
  (bind _asbpp_body_part (cast `/Game/Blueprints/Player/BPP_BodyPart` (`GameplayStatics.GetPlayerPawn` 0)))
  (cast `/Game/Blueprints/Player/BP_P_Torso` _asbpp_body_part
    (:`then`
      ; Si PawnCondition est vide, true par défaut
      (if (and (not (`BlueprintMapLibrary.Map_IsEmpty` _pawnconditions)) (or _value_4 _value_5 _value_3 _value_2 _value))
        ;;[0.4167 0.4167 0.4167 0.5] It returns false only when pawn conditions is true and the pawn does not contain the required bodypart (But it looks like shit thanks to Blueprint
        (if (not _value_4)
          (bind _bodypartsinpawn (`/Game/Blueprints/Player/BPP_BodyPart.bodyPartsInPawn` _asbpp_body_part))
          (bind _output (`|GetArrayItem` _bodypartsinpawn 2))
          (bind _output_2 (`|GetArrayItem` _bodypartsinpawn 3))
          (if (and (or _output _output_2) _value_5 true) :!label _label
            _
            (elif (not (and (and _output _output_2) _value_3 true))
              (bind _output_3 (`|GetArrayItem` _bodypartsinpawn 4))
              (bind _output_4 (`|GetArrayItem` _bodypartsinpawn 5))
              (if (and (or _output_3 _output_4) _value_2 true)
                _
                (elif (and (and _output_3 _output_4) _value true)
                  _
                  (else
                    (return false)))))))))
    (:`CastFailed`
      (goto _label)))
  (return true))

(fn `HoverBox`
  (bind _outlinematerialinstance (`self.OutlineMaterialInstance`))
  (`MaterialInstanceDynamic.SetScalarParameterValue` _outlinematerialinstance "Visibility" 1.0)
  (`MaterialInstanceDynamic.SetScalarParameterValue` _outlinematerialinstance "ComplexOutline" 1.0))

(fn `InitGameInstance`
  (bind _asbp_gi_ew_game_instance (cast `/Game/Blueprints/Managing/BP_GI_EwGameInstance` (`GameplayStatics.GetGameInstance`)))
  (set `self.Game Instance` _asbp_gi_ew_game_instance))

(fn `PlayPushSFX`
  (bind (_returnvalue_location _returnvalue_rotation) (`KismetMathLibrary.BreakTransform` (`self.GetTransform` self)))
  (`/Engine/EditorBlueprintResources/StandardMacros.IsValid` (`self.CrateAudioConst`)
    (:`Is Not Valid`
      (bind _returnvalue (`GameplayStatics.SpawnSoundAtLocation` (`BlueprintMapLibrary.Map_Find` (`/Game/Blueprints/Managing/BP_GI_EwGameInstance.InteractiveSoundCues` (`self.Game Instance`)) "NewEnumerator18") _returnvalue_location _returnvalue_rotation 1.0 1.0 0.0 "/Game/Audio/Settings/Attenuation_Interactive_Settings.Attenuation_Interactive_Settings" "/Game/Audio/Settings/Concurrency_Test_Settings.Concurrency_Test_Settings"))
      (set `self.CrateAudioConst` _returnvalue))))

(fn `SaveMaterialColor`
  (switch `/Game/Utilities/EMaterialColor` (`self.Material Color`)
    (:`NewEnumerator0`
      (set `self.Material to Apply` "/Game/Assets/Materials/Material_Puzzle/Materiaux_Triggers/MI_Triggers_Blanc.MI_Triggers_Blanc"))
    (:`NewEnumerator1`
      (set `self.Material to Apply` "/Game/Assets/Materials/Material_Puzzle/Materiaux_Triggers/MI_Triggers_Bleu.MI_Triggers_Bleu"))
    (:`NewEnumerator2`
      (set `self.Material to Apply` "/Game/Assets/Materials/Material_Puzzle/Materiaux_Triggers/MI_Triggers_Orange.MI_Triggers_Orange"))
    (:`NewEnumerator3`
      (set `self.Material to Apply` "/Game/Assets/Materials/Material_Puzzle/Materiaux_Triggers/MI_Triggers_Rose.MI_Triggers_Rose"))
    (:`NewEnumerator4`
      (set `self.Material to Apply` "/Game/Assets/Materials/Material_Puzzle/Materiaux_Triggers/MI_Triggers_Rouge.MI_Triggers_Rouge"))
    (:`NewEnumerator5`
      (set `self.Material to Apply` "/Game/Assets/Materials/Material_Puzzle/Materiaux_Triggers/MI_Triggers_Vert.MI_Triggers_Vert"))))

(fn `StopPushSFX`
  (bind _crateaudioconst (`self.CrateAudioConst`))
  (`/Engine/EditorBlueprintResources/StandardMacros.IsValid` _crateaudioconst
    (:`Is Valid`
      (`AudioComponent.FadeOut` _crateaudioconst 0.2 0.0 "Linear"))))

(fn `UnHoverBox`
  (bind _outlinematerialinstance (`self.OutlineMaterialInstance`))
  (`MaterialInstanceDynamic.SetScalarParameterValue` _outlinematerialinstance "Visibility" 0.0)
  (`MaterialInstanceDynamic.SetScalarParameterValue` _outlinematerialinstance "ComplexOutline" 0.0))

(fn `UpdatePlayerAbove`
  (if (`KismetArrayLibrary.Array_IsEmpty` (`self.PlayerAbove`))
    _))

(fn `UserConstructionScript`
  (if (not (`self.Islounge`))
    (`self.SaveMaterialColor`)
    (`self.ApplyMaterialColor`)))