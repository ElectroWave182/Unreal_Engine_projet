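; Bounce floor actor that springs body-part characters and BP_A_PushFinal objects upward when they overlap its box.
; Body parts play a sound through the cached game instance and get an additive launch from their absolute vertical speed times BounceCoeff.
; Push objects instead have their physics velocity replaced by a purely vertical one from a stored VelocityObject value times the same coefficient.
; Both paths print debug values.
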(event `self.ReceiveBeginPlay`
  (`self.InitGameInstance`))

(event `self.Box.OnComponentBeginOverlap`
  (params (OverlappedComponent :type "PrimitiveComponent Object Reference") (OtherActor :type "Actor Object Reference") (OtherComp :type "PrimitiveComponent Object Reference") (OtherBodyIndex :type Integer) (bFromSweep :type Boolean) (SweepResult :type "HitResult Structure (by ref)"))
  (bind _returnvalue (`KismetMathLibrary.MakeVector` 0.0 0.0 (* (.z (`self.VelocityObject`)) (`self.BounceCoeff`))))
  (bind _asbpp_body_part (cast `/Game/Blueprints/Player/BPP_BodyPart` OtherActor)
    (:`then`
      (`self.PlaySFX`)
      (bind _returnvalue_2 (`KismetMathLibrary.Abs` (.z (`self.GetVelocity` _asbpp_body_part))))
      (bind _returnvalue_3 (* _returnvalue_2 (`self.BounceCoeff`)))
      (`Character.LaunchCharacter` _asbpp_body_part (`KismetMathLibrary.MakeVector` 0.0 0.0 _returnvalue_3) false false)
      (`KismetSystemLibrary.PrintString` (`KismetStringLibrary.Conv_DoubleToString` _returnvalue_2) true true (struct :`G` 0.66 :`B` 1.0 :`A` 1.0) 5.0)
      (`KismetSystemLibrary.PrintString` (`KismetStringLibrary.Conv_DoubleToString` _returnvalue_3)))
    (:`CastFailed`
      (bind _asbp_a_push_final (cast `/Game/Blueprints/Interactive/Stale/BP_A_PushFinal` OtherActor))
      (`PrimitiveComponent.SetPhysicsLinearVelocity` (`/Game/Blueprints/Interactive/Stale/BP_A_PushFinal.Object` _asbp_a_push_final) _returnvalue false "None")
      (`KismetSystemLibrary.PrintString` (`KismetStringLibrary.Conv_VectorToString` _returnvalue)))))

(fn `InitGameInstance`
  (bind _asbp_gi_ew_game_instance (cast `/Game/Blueprints/Managing/BP_GI_EwGameInstance` (`GameplayStatics.GetGameInstance`)))
  (set `self.Game Instance` _asbp_gi_ew_game_instance))

(fn `PlaySFX`
  (bind _game_instance (`self.Game Instance`))
  (`/Engine/EditorBlueprintResources/StandardMacros.IsValid` _game_instance
    (:`Is Valid`
      (`/Game/Blueprints/Managing/BP_GI_EwGameInstance.PlayInteractiveSound` _game_instance self "NewEnumerator19"))))

(fn `UserConstructionScript`)