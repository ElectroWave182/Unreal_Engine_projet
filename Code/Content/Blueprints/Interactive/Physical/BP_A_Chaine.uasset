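; Swingable physics chain that catches an overlapping BPP_BodyPart pawn with an arm, one pawn at a time.
; Hooking transfers the pawn's momentum to the last tagged link, attaches it there with movement and collision disabled, and eases it into place by timeline.
; Swing input pushes the link along camera forward, weighted by lever arm and mass, while turning the pawn.
; Release launches the pawn with capped link velocity, then delays re-hooking.
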(event `self.ReceiveBeginPlay`
  ;[0.7083 0.7083 0.7083 0.5] Vitesse des animations
  (`TimelineComponent.SetPlayRate` (`self.tempsPosition`) 2.0)
  (`TimelineComponent.SetPlayRate` (`self.tempsRotation`) 2.0))

(event `self.ReceiveActorBeginOverlap`
  (params (OtherActor :type "Actor Object Reference"))
  (bind _asbpp_body_part (cast `/Game/Blueprints/Player/BPP_BodyPart` OtherActor))
  (`self.accrocher` _asbpp_body_part))

(event `accrocher`
  (params (membre :type "/Game/Blueprints/Player/BPP_BodyPart Object Reference"))
  (bind _bodypartsinpawn (`/Game/Blueprints/Player/BPP_BodyPart.bodyPartsInPawn` membre))
  ;[0.6638 0.6638 0.6638 0.5] Accroche la partie du corps proche à la chaîne, s'il n'y en a pas déjà une
  (if (and (or (`|GetArrayItem` _bodypartsinpawn 2) (`|GetArrayItem` _bodypartsinpawn 3)) (`KismetStringLibrary.EqualEqual_StrStr` (`self.etat`) "decroche"))
    (set `self.etat` "accroche")
    (bind _output_get (set `self.pawnHooked` membre))
    (`/Game/Blueprints/Player/BPP_BodyPart.tenir` _output_get self)
    (`self.trouverMaillon`)
    (`self.attacher`)
    ;[0.7031 0.7031 0.7031 0.5] Positionne le personnage en bas de la chaîne
    (`self.recupererPositionEntree`)
    (bind (_direction _pawnlocation) (`Timeline|tempsPosition` :!label _label)
      (:`Update`
        (`self.recupererPositionSurChaine`)
        (`self.K2_SetActorLocation` (`self.pawnHooked`) (`KismetMathLibrary.VLerp` (`self.positionEntree`) (`self.positionSurChaine`) _pawnlocation) false false))
      (:`Finished`
        (`self.arreterAnimationPoistion`)))))

(event `arreterAnimationPoistion`
  ;[0.7031 0.7031 0.7031 0.5] Positionne le personnage en bas de la chaîne
  (`self.recupererPositionEntree`)
  (goto _label :!via `SetNewTime`))

(event `lacher`
  (params (membre :type "/Game/Blueprints/Player/BPP_BodyPart Object Reference (by ref)"))
  ;[0.7604 0.7604 0.7604 0.5] Détache la partie du corps attachée à la chaîne, si elle est contrôlée par le joueur
  (if (and (== membre (`self.pawnHooked`)) (`KismetStringLibrary.EqualEqual_StrStr` (`self.etat`) "accroche"))
    (set `self.etat` "enDecrochage")
    (`/Game/Blueprints/Player/BPP_BodyPart.tenir` (`self.pawnHooked`) null)
    (`self.detacher`)
    (`self.arreterAnimationRotation`)
    ;[0.7917 0.7917 0.7917 0.5] Libère la partie du corps attachée, si elle sort de la zone de la chaîne
    (`KismetSystemLibrary.Delay` 1.0)
    (set `self.etat` "decroche")
    (set `self.pawnHooked` null)))

(event `changerMembre`
  (params (nouveauMembre :type "/Game/Blueprints/Player/BPP_BodyPart Object Reference"))
  ;[0.7105 0.7105 0.7105 0.5] Remplace la partie du corps attachée à la chaîne par une autre
  (if (and (!= "/Game/Blueprints/Player/BPP_BodyPart.BPP_BodyPart" (`self.pawnHooked`)) (`KismetStringLibrary.EqualEqual_StrStr` (`self.etat`) "accroche"))
    (`self.detacher`))
  (set `self.etat` "decroche")
  (`self.accrocher` nouveauMembre))

(event `bouger`
  (params (membre :type "/Game/Blueprints/Player/BPP_BodyPart Object Reference (by ref)") (sens :type "Float (double-precision) (by ref)"))
  ;[0.7552 0.7552 0.7552 0.5] Fait bouger la chaîne là où le personnage est attaché
  (if (and (== membre (`self.pawnHooked`)) (`KismetStringLibrary.EqualEqual_StrStr` (`self.etat`) "accroche") (!= 0.0 sens))
    (`self.mouvoir` sens)
    ;[0.6875 0.6875 0.6875 0.5] Pivote le personnage dans la direction du mouvement
    (`|ExecutionSequence`
      (:`then_0`
        (bind (_direction _pawnrotation) (`Timeline|tempsRotation` :!label _label_2)
          (:`Update`
            (`self.tourner` _pawnrotation))))
      (:`then_1`
        (if (!= (`self.sensMouvement`) sens)
          (set `self.sensMouvement` sens)
          (goto _label_2 :!via `SetNewTime`))))))

(event `arreterAnimationRotation`
  ;[0.6875 0.6875 0.6875 0.5] Pivote le personnage dans la direction du mouvement
  (goto _label_2 :!via `Stop`))

(fn `attacher`
  (locals (positionAatteindre :type "Vector Structure"))
  (bind _pawnhooked (`self.pawnHooked`))
  (bind _pawnhooked_2 (`self.pawnHooked`))
  (bind _rootcomponent (`Actor.RootComponent` _pawnhooked_2))
  (`self.transfertJoueurChaine`)
  (`CharacterMovementComponent.DisableMovement` (`Character.CharacterMovement` _pawnhooked))
  (`PrimitiveComponent.SetCollisionEnabled` (`Character.CapsuleComponent` _pawnhooked) "NoCollision")
  ;[0.7292 0.7292 0.7292 0.5] Pivote le joueur dans le sens du balancement : vers l'avant (X positif) de la chaîne
  (`SceneComponent.SetAbsolute` _rootcomponent false true false)
  (`SceneComponent.K2_SetWorldRotation` _rootcomponent (`KismetMathLibrary.Conv_VectorToRotator` (`SceneComponent.GetForwardVector` (`self.DefaultSceneRoot`))) false false)
  (`self.K2_AttachToComponent` _pawnhooked_2 (`self.maillonAttache`) "None" "KeepWorld" "KeepWorld" "KeepWorld" true))

(fn `detacher`
  (bind _pawnhooked (`self.pawnHooked`))
  (`CharacterMovementComponent.SetMovementMode` (`Character.CharacterMovement` _pawnhooked) "MOVE_Falling" 0)
  (`self.K2_DetachFromActor` _pawnhooked "KeepWorld" "KeepWorld" "KeepWorld")
  (`PrimitiveComponent.SetCollisionEnabled` (`Character.CapsuleComponent` _pawnhooked) "QueryAndPhysics")
  (`self.transfertChaineJoueur`))

(fn `hasPawnHooked`
  (returns (estAccroche :type Boolean))
  (return (`KismetStringLibrary.EqualEqual_StrStr` (`self.etat`) "accroche")))

(fn `mouvoir`
  (params (sens :type "Float (double-precision)" :default 1.0))
  (locals (direction :type "Vector Structure"))
  (bind _pawnhooked (`self.pawnHooked`))
  (bind (_returnvalue_x _returnvalue_y _returnvalue_z) (`KismetMathLibrary.BreakVector` (`SceneComponent.K2_GetComponentLocation` (`self.DefaultSceneRoot`))))
  (bind (_returnvalue_x_2 _returnvalue_y_2 _returnvalue_z_2) (`KismetMathLibrary.BreakVector` (`SceneComponent.K2_GetComponentLocation` (`Actor.RootComponent` _pawnhooked))))
  (bind (_returnvalue_x_3 _returnvalue_y_3) (`KismetMathLibrary.BreakVector` (`SceneComponent.GetForwardVector` (`/Game/Blueprints/Player/BPP_BodyPart.FollowCamera` (`self.pawnHooked`)))))
  ;[0.75 0.75 0.75 0.5] Exerce une force selon une direction et une amplitude prédéfinies
  (bind _output_get (set `self.directionMouvement` (* sens (`KismetMathLibrary.MakeVector` _returnvalue_x_3 _returnvalue_y_3))))
  (`PrimitiveComponent.AddForce` (`self.maillonAttache`) (* _output_get (`self.amplitudeMouvement`) (- _returnvalue_z _returnvalue_z_2) (`/Game/Blueprints/Player/BPP_BodyPart.customMass` _pawnhooked)) "None" false))

(fn `recupererPositionEntree`
  (set `self.positionEntree` (`SceneComponent.K2_GetComponentLocation` (`Actor.RootComponent` (`self.pawnHooked`)))))

(fn `recupererPositionSurChaine`
  (bind _maillonattache (`self.maillonAttache`))
  ;[0.6927 0.6927 0.6927 0.5] Positionnement du joueur juste derrière la chaîne
  (set `self.positionSurChaine` (- (`SceneComponent.K2_GetComponentLocation` _maillonattache) (`KismetMathLibrary.GreaterGreater_VectorRotator` (+ (`.BoxExtent` (`KismetSystemLibrary.GetComponentBounds` _maillonattache)) (25.0 0.0 50.0)) (`SceneComponent.K2_GetComponentRotation` (`Actor.RootComponent` (`self.pawnHooked`)))))))

(fn `tourner`
  (params (temps :type "Float (single-precision)"))
  (bind _rootcomponent (`Actor.RootComponent` (`self.pawnHooked`)))
  ;[0.7604 0.7604 0.7604 0.5] Interpolation entre l'orientation actuelle du personnage, et celle du mouvement
  (`SceneComponent.K2_SetWorldRotation` _rootcomponent (`KismetMathLibrary.RLerp` (`SceneComponent.K2_GetComponentRotation` _rootcomponent) (`KismetMathLibrary.Conv_VectorToRotator` (`self.directionMouvement`)) (`local.temps`) true) false false))

(fn `transfertChaineJoueur`
  (locals (vitesse :type "Vector Structure"))
  (bind _output_get (set `local.vitesse` (* (`SceneComponent.GetComponentVelocity` (`self.maillonAttache`)) (`self.amplitudeSortie`))))
  ;[0.6719 0.6719 0.6719 0.5] Norme de la vitesse capée à amplitudeMax
  (if (not (> (`self.amplitudeSortieMax`) (`KismetMathLibrary.VSize` _output_get)))
    (set `local.vitesse` (* (`self.amplitudeSortieMax`) (`KismetMathLibrary.Normal` (`local.vitesse`)))))
  (`Character.LaunchCharacter` (`self.pawnHooked`) (`local.vitesse`) true true))

(fn `transfertJoueurChaine`
  (bind _pawnhooked (`self.pawnHooked`))
  (bind (_returnvalue_x _returnvalue_y _returnvalue_z) (`KismetMathLibrary.BreakVector` (`SceneComponent.K2_GetComponentLocation` (`self.DefaultSceneRoot`))))
  (bind (_returnvalue_x_2 _returnvalue_y_2 _returnvalue_z_2) (`KismetMathLibrary.BreakVector` (`SceneComponent.K2_GetComponentLocation` (`Actor.RootComponent` _pawnhooked))))
  ;[0.6823 0.6823 0.6823 0.5] Répercute la force du personnage sur la plateforme, pondérée par le bras de levier
  (`PrimitiveComponent.AddForce` (`self.maillonAttache`) (* (- _returnvalue_z _returnvalue_z_2) (`self.impact`) (`self.GetVelocity` _pawnhooked) (`/Game/Blueprints/Player/BPP_BodyPart.customMass` _pawnhooked)) "None" false))

(fn `trouverMaillon`
  (locals (numMaillon :type Integer))
  (bind _returnvalue (`self.GetComponentsByTag` "/Script/Engine.StaticMeshComponent" "maillon"))
  ;[0.2699 1 0.4172 0.5] Prend le dernier maillon
  (set `local.numMaillon` (`KismetArrayLibrary.Array_Length` _returnvalue))
  (set `self.maillonAttache` (`|GetArrayItem` _returnvalue (- (`local.numMaillon`) 1))))

(fn `UserConstructionScript`)