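; Breakable plate actor that the leg character or a falling pushable can smash, with an optional reinforced variant.
; Upper and lower box overlaps test stomps and gravity-aware charged jumps from underneath; reinforcement blocks charged jumps and demands stronger stomps or longer pushable drops.
; Breaking hides the cube, disables collision and plays a sound.
; When Duration is non-zero, leaving the upper box starts a delayed respawn.
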(event `self.ReceiveBeginPlay`
  (`self.InitGameInstance`))

(event `self.LowerBox.OnComponentBeginOverlap`
  (params (OverlappedComponent :type "PrimitiveComponent Object Reference") (OtherActor :type "Actor Object Reference") (OtherComp :type "PrimitiveComponent Object Reference") (OtherBodyIndex :type Integer) (bFromSweep :type Boolean) (SweepResult :type "HitResult Structure (by ref)"))
  ; Process stomping
  (`self.CheckIfStomp` OtherActor OverlappedComponent))

(event `self.UpperBox.OnComponentBeginOverlap`
  (params (OverlappedComponent :type "PrimitiveComponent Object Reference") (OtherActor :type "Actor Object Reference") (OtherComp :type "PrimitiveComponent Object Reference") (OtherBodyIndex :type Integer) (bFromSweep :type Boolean) (SweepResult :type "HitResult Structure (by ref)"))
  ; Process stomping
  (`self.CheckIfStomp` OtherActor OverlappedComponent))

(event `self.UpperBox.OnComponentEndOverlap`
  (params (OverlappedComponent :type "PrimitiveComponent Object Reference") (OtherActor :type "Actor Object Reference") (OtherComp :type "PrimitiveComponent Object Reference") (OtherBodyIndex :type Integer))
  (bind _cube (`self.Cube`))
  ; Respawn of the Fragile Plate
  (if (`self.IsBroken`)
    (if (!= (`self.Duration`) 0.0)
      (`KismetSystemLibrary.Delay` (`self.Duration`))
      (`PrimitiveComponent.SetCollisionEnabled` _cube "QueryAndPhysics")
      (`PrimitiveComponent.SetMaterial` _cube 0 "/Game/StarterContent/Materials/M_Glass.M_Glass")
      (`SceneComponent.SetVisibility` _cube true false)
      (set `self.IsBroken` false)
      (`KismetSystemLibrary.Delay` 0.5)
      (`PrimitiveComponent.SetMaterial` _cube 0 null))))

(fn `CheckIfStomp`
  (params (Actor :type "Actor Object Reference") (Box :type "PrimitiveComponent Object Reference"))
  (bind _returnvalue (== Box (`self.LowerBox`)))
  (bind _asbpp_p_leg (cast `/Game/Blueprints/Player/BPP_P_Leg` Actor)
    (:`then`
      (bind (_returnvalue_x _returnvalue_y _returnvalue_z) (`KismetMathLibrary.BreakVector` (`CharacterMovementComponent.GetGravityDirection` (`Character.CharacterMovement` _asbpp_p_leg))))
      (if (and _returnvalue (== _returnvalue_z -1.0))
        ; Charged jump check
        (if (and (`/Game/Blueprints/Player/BPP_P_Leg.IsChargedJump` _asbpp_p_leg) (not (`self.IsReinforced`))) :!label _label
          (set `/Game/Blueprints/Player/BPP_P_Leg.IsChargedJump` false _asbpp_p_leg)
          (`self.DestroyPlate` :!label _label_2)
          (`self.PlaySFX` "NewEnumerator20")
          (else
            ; Stomp check
            (if (and (`/Game/Blueprints/Player/BPP_P_Leg.IsStomping` _asbpp_p_leg) (not (`self.IsBroken`))) :!label _label_3
              (bind _chargedstomp (`/Game/Blueprints/Player/BPP_P_Leg.processStompMagnitude` _asbpp_p_leg))
              (if (`self.IsReinforced`)
                (if _chargedstomp
                  (goto _label_2))
                (else
                  (goto _label_2))))))
        (elif (and (not _returnvalue) (== _returnvalue_z 1.0))
          (goto _label)
          (else
            (goto _label_3)))))
    (:`CastFailed`
      ; Stomp from Pushable
      (bind _asbp_a_pushable (cast `/Game/Blueprints/Interactive/Physical/BP_A_Pushable` Actor))
      (if (`self.IsReinforced`)
        (bind (_initposition_x _initposition_y _initposition_z) (`KismetMathLibrary.BreakVector` (`/Game/Blueprints/Interactive/Physical/BP_A_Pushable.InitPosition` _asbp_a_pushable)))
        (bind (_returnvalue_x_2 _returnvalue_y_2 _returnvalue_z_2) (`KismetMathLibrary.BreakVector` (`self.K2_GetActorLocation` _asbp_a_pushable)))
        (bind _returnvalue_2 (`KismetMathLibrary.Abs` (- _initposition_z _returnvalue_z_2)))
        (if (> _returnvalue_2 590.0)
          (goto _label_2))
        (elif (> _returnvalue_2 390.0)
          (goto _label_2))))))

(fn `DestroyPlate`
  (bind _cube (`self.Cube`))
  ; Destruction of the plate
  (`PrimitiveComponent.SetCollisionEnabled` _cube "NoCollision")
  (`PrimitiveComponent.SetMaterial` _cube 0 "/Game/StarterContent/Materials/M_Glass.M_Glass")
  (`SceneComponent.SetVisibility` _cube false false)
  (set `self.IsBroken` true))

(fn `isWeightSuffisient`
  (params (Object :type "Object Object Reference"))
  (returns (ReturnValue :type Boolean))
  (return false))

(fn `UserConstructionScript`)