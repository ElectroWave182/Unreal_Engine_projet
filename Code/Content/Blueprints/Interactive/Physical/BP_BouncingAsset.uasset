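; BP_BouncingAsset is an interactive physical prop that reacts with a bounce when something overlaps its box trigger.
; On BeginPlay it caches the BP_GI_EwGameInstance game instance.
; Each box overlap plays an interactive sound through that game instance, then calls BouncingEvent on its bouncing component, which handles the bounce itself.
; The overlap is not filtered by actor type.
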(event `self.ReceiveBeginPlay`
  (`self.InitGameInstance`))

(event `self.Box.OnComponentBeginOverlap`
  (params (OverlappedComponent :type "PrimitiveComponent Object Reference") (OtherActor :type "Actor Object Reference") (OtherComp :type "PrimitiveComponent Object Reference") (OtherBodyIndex :type Integer) (bFromSweep :type Boolean) (SweepResult :type "HitResult Structure (by ref)"))
  (`self.PlaySFX`)
  (`/Game/Blueprints/Interactive/Physical/BPC_BouncingComponent.BouncingEvent` (`self.BPC_BouncingComponent`)))

(fn `InitGameInstance`
  (bind _asbp_gi_ew_game_instance (cast `/Game/Blueprints/Managing/BP_GI_EwGameInstance` (`GameplayStatics.GetGameInstance`)))
  (set `self.Game Instance` _asbp_gi_ew_game_instance))

(fn `PlaySFX`
  (bind _game_instance (`self.Game Instance`))
  (`/Engine/EditorBlueprintResources/StandardMacros.IsValid` _game_instance
    (:`Is Valid`
      (`/Game/Blueprints/Managing/BP_GI_EwGameInstance.PlayInteractiveSound` _game_instance self "NewEnumerator19"))))

(fn `UserConstructionScript`)