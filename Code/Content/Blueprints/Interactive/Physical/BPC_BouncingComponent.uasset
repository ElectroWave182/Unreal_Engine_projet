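; BPC_BouncingComponent is a component that bounces the player character vertically.
; Its BouncingEvent launches player 0 upward by the absolute Z velocity times BounceCoeff, leaving horizontal motion intact.
; The launch adds to current velocity rather than overriding it, so a falling character needs a coefficient above 1 to rebound.
; It prints speed and scaled value for debugging, and nothing in this graph calls the event.
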(event `BouncingEvent`
  (bind _returnvalue (`KismetMathLibrary.Abs` (.z (`Actor.GetVelocity` (`GameplayStatics.GetPlayerCharacter` 0)))))
  (bind _returnvalue_2 (* _returnvalue (`self.Bounce coeff`)))
  (`Character.LaunchCharacter` (`GameplayStatics.GetPlayerCharacter` 0) (`KismetMathLibrary.MakeVector` 0.0 0.0 _returnvalue_2) false false)
  (`KismetSystemLibrary.PrintString` (`KismetStringLibrary.Conv_DoubleToString` _returnvalue) true true (struct :`G` 0.66 :`B` 1.0 :`A` 1.0) 5.0)
  (`KismetSystemLibrary.PrintString` (`KismetStringLibrary.Conv_DoubleToString` _returnvalue_2)))