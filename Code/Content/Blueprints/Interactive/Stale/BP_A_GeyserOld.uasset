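; Stale geyser actor meant to propel player body parts and pushables upward, with its launch logic left disconnected.
; A Signal/BeginPlay loop toggles it on optional timers, activating Niagara only while a body part is inside a proximity box to save performance.
; Construction sizes an entry capsule and larger exit capsule from max height.
; Overlap checks use line traces for blockers; exiting or deactivation stops animations and restores physics for tracked actors.
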(event `Propulsion`
  ; Start propulsion
)

(event `self.ReceiveSignal`
  (bind _activatetime (`self.ActivateTime`))
  (if (`self.state`) :!label _label
    ; Active Behavior
    (set `self.currentState` true)
    (`self.ActivateGeyser`)
    (if (not (== 0.0 _activatetime))
      (`KismetSystemLibrary.Delay` _activatetime)
      (set `self.currentState` false)
      (`self.DeactivateGeyser`)
      (`KismetSystemLibrary.Delay` (`self.GeyserInterval`))
      (goto _label))
    (else
      ; Deactive Behavior
      (set `self.currentState` false)
      (`self.DeactivateGeyser`))))

(event `self.ReceiveBeginPlay`
  (bind _capsuleentree (`self.CapsuleEntree`))
  (set `self.MaxHeigth` (* (- (`CapsuleComponent.GetScaledCapsuleHalfHeight` _capsuleentree) (`CapsuleComponent.GetScaledCapsuleRadius` _capsuleentree)) 2.0))
  (goto _label))

(event `self.CapsuleEntree.OnComponentBeginOverlap`
  (params (OverlappedComponent :type "PrimitiveComponent Object Reference") (OtherActor :type "Actor Object Reference") (OtherComp :type "PrimitiveComponent Object Reference") (OtherBodyIndex :type Integer) (bFromSweep :type Boolean) (SweepResult :type "HitResult Structure (by ref)"))
  ; Actor tracking
  (bind _apropulser (`self.CheckIfOverlaps` OverlappedComponent OtherActor))
  (if _apropulser
    (`self.goIn` OtherActor)))

(event `goIn`
  (params (acteur :type "Actor Object Reference"))
  ; Actor tracking
)

(event `self.CapsuleEntree.OnComponentEndOverlap`
  (params (OverlappedComponent :type "PrimitiveComponent Object Reference") (OtherActor :type "Actor Object Reference") (OtherComp :type "PrimitiveComponent Object Reference") (OtherBodyIndex :type Integer))
  ; Actor tracking
  (bind _apropulser (`self.CheckIfOverlaps` OverlappedComponent OtherActor))
  (if (not _apropulser)
    (`self.stopPropulsion` OtherActor)))

(event `goOut`
  (params (acteur :type "Actor Object Reference"))
  ; Actor tracking
)

(event `self.CapsuleSortie.OnComponentEndOverlap`
  (params (OverlappedComponent :type "PrimitiveComponent Object Reference") (OtherActor :type "Actor Object Reference") (OtherComp :type "PrimitiveComponent Object Reference") (OtherBodyIndex :type Integer))
  ; Actor tracking
  (bind _apropulser (`self.CheckIfOverlaps` OverlappedComponent OtherActor))
  (if (not _apropulser)
    (`self.takeOutActor` OtherActor)
    (`BlueprintSetLibrary.Set_Remove` (`self.overlappingActors`) OtherActor)))

(event `self.PlayerNearbyBounds.OnComponentBeginOverlap`
  (params (OverlappedComponent :type "PrimitiveComponent Object Reference") (OtherActor :type "Actor Object Reference") (OtherComp :type "PrimitiveComponent Object Reference") (OtherBodyIndex :type Integer) (bFromSweep :type Boolean) (SweepResult :type "HitResult Structure (by ref)"))
  ; Activate / Deactivate with distance to gain performance
  ;; Player enter geyser and it activates
  (if (and (`KismetMathLibrary.ClassIsChildOf` (`GameplayStatics.GetObjectClass` OtherActor) "/Game/Blueprints/Player/BPP_BodyPart.BPP_BodyPart_C") (not (`self.isPlayerNear`)))
    (set `self.isPlayerNear` true)
    (if (`self.state`)
      (`self.ActivateGeyser`))))

(event `self.PlayerNearbyBounds.OnComponentEndOverlap`
  (params (OverlappedComponent :type "PrimitiveComponent Object Reference") (OtherActor :type "Actor Object Reference") (OtherComp :type "PrimitiveComponent Object Reference") (OtherBodyIndex :type Integer))
  ; Activate / Deactivate with distance to gain performance
  ;; Player exit geyser and it deactivates
  (if (`KismetMathLibrary.ClassIsChildOf` (`GameplayStatics.GetObjectClass` OtherActor) "/Game/Blueprints/Player/BPP_BodyPart.BPP_BodyPart_C")
    (if (== (`KismetArrayLibrary.Array_Length` (`PrimitiveComponent.GetOverlappingActors` OverlappedComponent "/Game/Blueprints/Player/BPP_BodyPart.BPP_BodyPart_C")) 0)
      (set `self.isPlayerNear` false)
      (if (== 0.0 (`self.ActivateTime`))
        (`self.DeactivateGeyser`)))))

(fn `ActivateGeyser`
  (bind _niagara (`self.Niagara`))
  (if (`self.isPlayerNear`)
    (`ActorComponent.SetActive` _niagara true false)
    (`SceneComponent.SetVisibility` _niagara true false)
    (`PrimitiveComponent.SetCollisionEnabled` (`self.CapsuleEntree`) "QueryAndPhysics")
    (`self.Propulsion`)))

(fn `addActorAndAbove`
  (params (acteur :type "Actor Object Reference"))
  (bind _acteur (`local.acteur`))
  ;[0.6406 0.6406 0.6406 0.5] Cas récursif : on ajoute l'acteur s'il est pris en charge par le geyser
  (cast `/Game/Blueprints/Player/BPP_BodyPart` acteur
    (:`then`
      _)
    (:`CastFailed`
      (bind _asbp_a_pushable (cast `/Game/Blueprints/Interactive/Physical/BP_A_Pushable` acteur))
      (`|ExecutionSequence`
        (:`then_0`
          _))))
  (if (not (`BlueprintSetLibrary.Set_Contains` (`self.overlappingActors`) _acteur))
    (`BlueprintSetLibrary.Set_Add` (`self.overlappingActors`) _acteur)))

(fn `CheckIfBlock`
  (params (Other :type "Actor Object Reference"))
  (returns (isBlocked :type Boolean))
  (bind (_outhit _returnvalue) (`KismetSystemLibrary.LineTraceSingle` (`self.K2_GetActorLocation`) (`self.K2_GetActorLocation` Other) "TraceTypeQuery3" false (`|MakeArray` Other)))
  (return _returnvalue))

(fn `CheckIfOverlaps`
  (params (capsule :type "PrimitiveComponent Object Reference") (acteur :type "Actor Object Reference"))
  (returns (aPropulser :type Boolean))
  (bind _asbpp_body_part (cast `/Game/Blueprints/Player/BPP_BodyPart` acteur)
    (:`then`
      ; Check if player is above a Pushable
      (bind (_outhit _returnvalue) (`KismetSystemLibrary.LineTraceSingle` (`self.K2_GetActorLocation`) (`self.K2_GetActorLocation` _asbpp_body_part) "TraceTypeQuery1" false (`|MakeArray` _asbpp_body_part :!type "Actor Object Reference")))
      (if (not _returnvalue)
        ;[0.149 0.07843 0 0.502] Collision principale de la partie du corps
        (return (`PrimitiveComponent.IsOverlappingComponent` (`Character.CapsuleComponent` _asbpp_body_part) (`local.capsule`)))))
    (:`CastFailed`
      (bind _asbp_a_pushable (cast `/Game/Blueprints/Interactive/Physical/BP_A_Pushable` acteur)
        (:`then`
          ;[0.349 0 0.6627 0.502] Centre de l'objet poussable
          (return (`PrimitiveComponent.IsOverlappingComponent` (`/Game/Blueprints/Interactive/Physical/BP_A_Pushable.StepOn5` _asbp_a_pushable) (`local.capsule`))))
        (:`CastFailed`
          (return false))))))

(fn `DeactivateGeyser`
  (bind _niagara (`self.Niagara`))
  (`ActorComponent.SetActive` _niagara false false)
  (`SceneComponent.SetVisibility` _niagara false false)
  (bind _result (`BlueprintSetLibrary.Set_ToArray` (`self.overlappingActors`)))
  (for _array_element _result
    (`self.takeOutActor` _array_element)))

(fn `stopPropulsion`
  (params (actor :type "Actor Object Reference"))
  (bind _asbpp_body_part (cast `/Game/Blueprints/Player/BPP_BodyPart` actor)
    (:`then`
      (`/Game/Blueprints/Player/BPP_BodyPart.StopAnim_Geyser` _asbpp_body_part))
    (:`CastFailed`
      (bind _asbp_a_pushable (cast `/Game/Blueprints/Interactive/Physical/BP_A_Pushable` actor))
      (`/Game/Blueprints/Interactive/Physical/BP_A_Pushable.StopAnim_Geyser` _asbp_a_pushable))))

(fn `takeOutActor`
  (params (actor :type "Actor Object Reference"))
  (if (`BlueprintSetLibrary.Set_Contains` (`self.overlappingActors`) actor)
    (bind _asbpp_body_part (cast `/Game/Blueprints/Player/BPP_BodyPart` actor)
      (:`then`
        ;[0.149 0.07843 0 0.502] Physique d'une partie du corps
        (`/Game/Blueprints/Player/BPP_BodyPart.StopAnim_Geyser` _asbpp_body_part)
        (bind _charactermovement (`Character.CharacterMovement` _asbpp_body_part))
        (set `CharacterMovementComponent.GravityScale` 1.75 _charactermovement)
        (set `CharacterMovementComponent.MaxAcceleration` 600.0 _charactermovement))
      (:`CastFailed`
        (bind _asbp_a_pushable (cast `/Game/Blueprints/Interactive/Physical/BP_A_Pushable` actor))
        ;[0.349 0 0.6627 0.502] Physique d'un objet poussable
        (`/Game/Blueprints/Interactive/Physical/BP_A_Pushable.StopAnim_Geyser` _asbp_a_pushable)
        (`PrimitiveComponent.SetEnableGravity` (`/Game/Blueprints/Interactive/Physical/BP_A_Pushable.BoxSkin` _asbp_a_pushable) true)))))

(fn `UserConstructionScript`
  (locals (rayonEntree :type "Float (double-precision)") (rayonSortie :type "Float (double-precision)"))
  (bind _playernearbysize (`self.PlayerNearbySize`))
  (bind _playernearbybounds (`self.PlayerNearbyBounds`))
  (bind _capsuleentree (`self.CapsuleEntree`))
  (bind _capsulesortie (`self.CapsuleSortie`))
  (bind _returnvalue (* (`self.MaxHeigth`) 50.0))
  (bind _returnvalue_2 (- (+ (`CapsuleComponent.GetUnscaledCapsuleHalfHeight` (`self.CapsuleEntree`)) (`local.rayonSortie`)) (`local.rayonEntree`)))
  (set `local.rayonEntree` (`CapsuleComponent.GetUnscaledCapsuleRadius` (`self.CapsuleEntree`)))
  (set `local.rayonSortie` (`CapsuleComponent.GetUnscaledCapsuleRadius` (`self.CapsuleSortie`)))
  ;[0.6311 0.6311 0.6311 0.5] Petite capsule pour les requêtes d'entrée
  (`CapsuleComponent.SetCapsuleHalfHeight` _capsuleentree (+ (`local.rayonEntree`) _returnvalue) false)
  (`SceneComponent.K2_SetRelativeLocation` _capsuleentree (`KismetMathLibrary.MakeVector` 0.0 0.0 _returnvalue) false false)
  ;[0.6825 0.6825 0.6825 0.5] Grande capsule pour les requêtes de sortie
  (`CapsuleComponent.SetCapsuleHalfHeight` _capsulesortie _returnvalue_2 false)
  (`SceneComponent.K2_SetRelativeLocation` _capsulesortie (`KismetMathLibrary.MakeVector` 0.0 0.0 (- _returnvalue_2 (`local.rayonSortie`))) false false)
  ;[0.6731 0.6731 0.6731 0.5] Grosse boîte anti-lag
  (`BoxComponent.SetBoxExtent` _playernearbybounds _playernearbysize false)
  (`SceneComponent.K2_SetRelativeLocation` _playernearbybounds (`KismetMathLibrary.MakeVector` 0.0 0.0 (+ (.z _playernearbysize) (`self.PlayerNearbyHeigth`))) false false))