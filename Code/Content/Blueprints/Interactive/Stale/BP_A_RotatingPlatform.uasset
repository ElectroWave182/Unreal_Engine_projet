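; Interactive rotating platform actor whose yaw motion is switched on and off by a signal state, evaluated on BeginPlay through ReceiveSignal.
; When State is true, the Chronologie timeline plays at the Speed rate and sets the root's relative yaw each update; otherwise it stops.
; Timeline time is derived from the stored yaw, and ChangeRotation stores a new rotation and calls SetNewTime on the timeline.
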(event `self.ReceiveBeginPlay`
  (`/Game/Blueprints/Interactive/Interfaces/BPI_ReceiveSignal.ReceiveSignal`))

(event `/Game/Blueprints/Interactive/Interfaces/BPI_ReceiveSignal.ReceiveSignal`
  (if (`self.state`)
    (`TimelineComponent.SetPlayRate` (`self.Chronologie`) (`self.Speed`))
    (bind (_direction _rotation) (`Timeline|Chronologie` :`NewTime` (/ (+ (.yaw (stale `/Game/Blueprints/Interactive/Interfaces/BPI_SignalsToReceiver.ChangeRotation` _output_get)) 90.0) 180.0) :!label _label)
      (:`Update`
        (bind _output_get (set `self.Rotation` (`KismetMathLibrary.MakeRotator` 0.0 0.0 _rotation)))
        (`SceneComponent.K2_SetRelativeRotation` (`self.DefaultSceneRoot`) _output_get false false)))
    (else
      (goto _label :!via `Stop`))))

(event `/Game/Blueprints/Interactive/Interfaces/BPI_SignalsToReceiver.ChangeRotation`
  (params (newRotation :type "Rotator Structure"))
  ;[0.7083 0.7083 0.7083 0.5] Change la rotation instantanément
  (bind _output_get (set `self.Rotation` newRotation))
  (goto _label :!via `SetNewTime`))

(fn `UserConstructionScript`)