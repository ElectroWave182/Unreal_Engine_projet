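; Pushable cube actor that simulates physics while a collision box on the X or Y axis is overlapped and the inherited pawn-condition check passes.
; A bottom collision overlap disables gravity and locks the physics constraint's Z axis, and ending it frees the axis so the cube falls.
; A downward line-trace fall check and some IsPushing setters remain in the graph but are disconnected.
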(event `self.Y Axis Collision.OnComponentBeginOverlap`
  (params (OverlappedComponent :type "PrimitiveComponent Object Reference") (OtherActor :type "Actor Object Reference") (OtherComp :type "PrimitiveComponent Object Reference") (OtherBodyIndex :type Integer) (bFromSweep :type Boolean) (SweepResult :type "HitResult Structure (by ref)"))
  ; Y Axis Collision
  (bind _isvalid (`self.CheckPawnConditions`))
  (if _isvalid
    (`PrimitiveComponent.SetSimulatePhysics` (`self.Cube`) true)))

(event `self.Y Axis Collision.OnComponentEndOverlap`
  (params (OverlappedComponent :type "PrimitiveComponent Object Reference") (OtherActor :type "Actor Object Reference") (OtherComp :type "PrimitiveComponent Object Reference") (OtherBodyIndex :type Integer))
  ; Y Axis Collision
  (bind _isvalid (`self.CheckPawnConditions`))
  (if _isvalid
    (`PrimitiveComponent.SetSimulatePhysics` (`self.Cube`) false)))

(event `self.X Axis Collision.OnComponentBeginOverlap`
  (params (OverlappedComponent :type "PrimitiveComponent Object Reference") (OtherActor :type "Actor Object Reference") (OtherComp :type "PrimitiveComponent Object Reference") (OtherBodyIndex :type Integer) (bFromSweep :type Boolean) (SweepResult :type "HitResult Structure (by ref)"))
  ; X Axis Collision
  (bind _isvalid (`self.CheckPawnConditions`))
  (if _isvalid
    (`PrimitiveComponent.SetSimulatePhysics` (`self.Cube`) true)))

(event `self.X Axis Collision.OnComponentEndOverlap`
  (params (OverlappedComponent :type "PrimitiveComponent Object Reference") (OtherActor :type "Actor Object Reference") (OtherComp :type "PrimitiveComponent Object Reference") (OtherBodyIndex :type Integer))
  ; X Axis Collision
  (bind _isvalid (`self.CheckPawnConditions`))
  (if _isvalid
    (`PrimitiveComponent.SetSimulatePhysics` (`self.Cube`) false)))

(event `self.Bottom Collision.OnComponentBeginOverlap`
  (params (OverlappedComponent :type "PrimitiveComponent Object Reference") (OtherActor :type "Actor Object Reference") (OtherComp :type "PrimitiveComponent Object Reference") (OtherBodyIndex :type Integer) (bFromSweep :type Boolean) (SweepResult :type "HitResult Structure (by ref)"))
  (`PrimitiveComponent.SetEnableGravity` (`self.Cube`) false)
  (set `self.IsFalling?` false)
  (`PhysicsConstraintComponent.SetLinearZLimit` (`self.PhysicsConstraint`) "LCM_Locked" 0.0))

(event `self.Bottom Collision.OnComponentEndOverlap`
  (params (OverlappedComponent :type "PrimitiveComponent Object Reference") (OtherActor :type "Actor Object Reference") (OtherComp :type "PrimitiveComponent Object Reference") (OtherBodyIndex :type Integer))
  (`PrimitiveComponent.SetEnableGravity` (`self.Cube`) true)
  (set `self.IsFalling?` true)
  (`PhysicsConstraintComponent.SetLinearZLimit` (`self.PhysicsConstraint`) "LCM_Free" 0.0))

(event `self.ReceiveTick`
  (params (DeltaSeconds :type "Float (single-precision)"))
  ; Marche pas trop
)

(fn `CheckPawnConditions`
  (returns (IsValid :type Boolean))
  (bind _isvalid (`parent.CheckPawnConditions`))
  (return _isvalid))

(fn `UserConstructionScript`)