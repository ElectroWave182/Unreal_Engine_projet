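; Pushable interactive actor that flags an overlapping BPP_BodyPart pawn as pushing.
; Two triggers, Box and Box1, run identical logic: if the inherited CheckPawnConditions passes, overlap begin disables physics on Box and sets IsPushing, and overlap end reverses both.
; A separate GroundCheck component toggles IsGround on any overlap, though this graph never reads that flag.
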(event `self.Box.OnComponentBeginOverlap`
  (params (OverlappedComponent :type "PrimitiveComponent Object Reference") (OtherActor :type "Actor Object Reference") (OtherComp :type "PrimitiveComponent Object Reference") (OtherBodyIndex :type Integer) (bFromSweep :type Boolean) (SweepResult :type "HitResult Structure (by ref)"))
  (bind _asbpp_body_part (cast `/Game/Blueprints/Player/BPP_BodyPart` OtherActor))
  (bind _isvalid (`self.CheckPawnConditions`))
  (if _isvalid
    (`PrimitiveComponent.SetSimulatePhysics` (`self.Box`) false)
    (set `/Game/Blueprints/Player/BPP_BodyPart.IsPushing?` true _asbpp_body_part)))

(event `self.Box.OnComponentEndOverlap`
  (params (OverlappedComponent :type "PrimitiveComponent Object Reference") (OtherActor :type "Actor Object Reference") (OtherComp :type "PrimitiveComponent Object Reference") (OtherBodyIndex :type Integer))
  (bind _asbpp_body_part (cast `/Game/Blueprints/Player/BPP_BodyPart` OtherActor))
  (bind _isvalid (`self.CheckPawnConditions`))
  (if _isvalid
    (`PrimitiveComponent.SetSimulatePhysics` (`self.Box`) true)
    (set `/Game/Blueprints/Player/BPP_BodyPart.IsPushing?` false _asbpp_body_part)))

(event `self.Box1.OnComponentBeginOverlap`
  (params (OverlappedComponent :type "PrimitiveComponent Object Reference") (OtherActor :type "Actor Object Reference") (OtherComp :type "PrimitiveComponent Object Reference") (OtherBodyIndex :type Integer) (bFromSweep :type Boolean) (SweepResult :type "HitResult Structure (by ref)"))
  (bind _asbpp_body_part (cast `/Game/Blueprints/Player/BPP_BodyPart` OtherActor))
  (bind _isvalid (`self.CheckPawnConditions`))
  (if _isvalid
    (`PrimitiveComponent.SetSimulatePhysics` (`self.Box`) false)
    (set `/Game/Blueprints/Player/BPP_BodyPart.IsPushing?` true _asbpp_body_part)))

(event `self.Box1.OnComponentEndOverlap`
  (params (OverlappedComponent :type "PrimitiveComponent Object Reference") (OtherActor :type "Actor Object Reference") (OtherComp :type "PrimitiveComponent Object Reference") (OtherBodyIndex :type Integer))
  (bind _asbpp_body_part (cast `/Game/Blueprints/Player/BPP_BodyPart` OtherActor))
  (bind _isvalid (`self.CheckPawnConditions`))
  (if _isvalid
    (`PrimitiveComponent.SetSimulatePhysics` (`self.Box`) true)
    (set `/Game/Blueprints/Player/BPP_BodyPart.IsPushing?` false _asbpp_body_part)))

(event `self.GroundCheck.OnComponentBeginOverlap`
  (params (OverlappedComponent :type "PrimitiveComponent Object Reference") (OtherActor :type "Actor Object Reference") (OtherComp :type "PrimitiveComponent Object Reference") (OtherBodyIndex :type Integer) (bFromSweep :type Boolean) (SweepResult :type "HitResult Structure (by ref)"))
  (set `self.IsGround?` true))

(event `self.GroundCheck.OnComponentEndOverlap`
  (params (OverlappedComponent :type "PrimitiveComponent Object Reference") (OtherActor :type "Actor Object Reference") (OtherComp :type "PrimitiveComponent Object Reference") (OtherBodyIndex :type Integer))
  (set `self.IsGround?` false))

(fn `CheckPawnConditions`
  (returns (IsValid :type Boolean))
  (bind _isvalid (`parent.CheckPawnConditions`))
  (return _isvalid))

(fn `UserConstructionScript`)