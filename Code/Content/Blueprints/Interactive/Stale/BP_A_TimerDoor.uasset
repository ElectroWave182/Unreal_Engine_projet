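; Timer door actor that slides its Door component vertically and closes it again after a cooldown.
; Signal plays a timeline when State is true, lerping the door's relative Z up to ZDifference, and reverses it otherwise.
; A Delay hung off the timeline's Update clears State and reverses the timeline after CooldownDuration.
; Nothing in this graph sets State back to true.
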(event `self.ReceiveSignal`
  (if (`self.state`)
    ; Animation managing
    (bind (_direction _opennig_door) (`Timeline|Door Timeline_0` :!label _label)
      (:`Update`
        (`SceneComponent.K2_SetRelativeLocation` (`self.door`) (`KismetMathLibrary.MakeVector` 0.0 0.0 (`KismetMathLibrary.Lerp` 0.0 (`self.ZDifference`) _opennig_door)) false false)
        ; Reset managing
        (`KismetSystemLibrary.Delay` (`self.cooldownDuration`))
        (if (`self.state`)
          (set `self.state` false)
          (goto _label :!via `Reverse`))))
    (else
      (goto _label :!via `Reverse`))))

(fn `UserConstructionScript`)