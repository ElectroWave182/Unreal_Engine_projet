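; Trigger volume that blacks out the player's view while their controlled body part is inside, unless it is a torso with at least one eye.
; Box overlaps maintain a list of body parts inside and update the manual camera fade using the game instance's controlled part, with debug prints on entry.
; Tick also reapplies the fade every frame, checking the player character against that list.
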(event `self.ReceiveTick`
  (params (DeltaSeconds :type "Float (single-precision)"))
  (bind _asbpp_body_part (cast `/Game/Blueprints/Player/BPP_BodyPart` (`GameplayStatics.GetPlayerCharacter` 0)))
  (if (`KismetArrayLibrary.Array_Contains` (`self.MembresAffectés`) _asbpp_body_part)
    (bind _asbp_p_torso (cast `/Game/Blueprints/Player/BP_P_Torso` _asbpp_body_part)
      (:`then`
        (if (>= (`/Game/Blueprints/Player/BPP_BodyPart.eyeCount` _asbp_p_torso) 1)
          (`PlayerCameraManager.SetManualCameraFade` :`self` (`PlayerController.PlayerCameraManager` (`GameplayStatics.GetPlayerController` 0)))
          (else
            (`PlayerCameraManager.SetManualCameraFade` :`self` (`PlayerController.PlayerCameraManager` (`GameplayStatics.GetPlayerController` 0)) :`InFadeAmount` 1.0))))
      (:`CastFailed`
        (`PlayerCameraManager.SetManualCameraFade` :`self` (`PlayerController.PlayerCameraManager` (`GameplayStatics.GetPlayerController` 0)) :`InFadeAmount` 1.0)))
    (else
      (`PlayerCameraManager.SetManualCameraFade` :`self` (`PlayerController.PlayerCameraManager` (`GameplayStatics.GetPlayerController` 0))))))

(event `self.Box.OnComponentBeginOverlap`
  (params (OverlappedComponent :type "PrimitiveComponent Object Reference") (OtherActor :type "Actor Object Reference") (OtherComp :type "PrimitiveComponent Object Reference") (OtherBodyIndex :type Integer) (bFromSweep :type Boolean) (SweepResult :type "HitResult Structure (by ref)"))
  (bind _asbpp_body_part (cast `/Game/Blueprints/Player/BPP_BodyPart` OtherActor)
    (:`then`
      (bind _returnvalue (`KismetArrayLibrary.Array_Add` (`self.MembresAffectés`) _asbpp_body_part))
      (`KismetSystemLibrary.PrintText` (`KismetTextLibrary.Conv_IntToText` _returnvalue))
      (bind _asbp_gi_ew_game_instance (cast `/Game/Blueprints/Managing/BP_GI_EwGameInstance` (`GameplayStatics.GetGameInstance`)))
      (if (`KismetArrayLibrary.Array_Contains` (`self.MembresAffectés`) (`/Game/Blueprints/Managing/BP_GI_EwGameInstance.CurrentControlledPart` _asbp_gi_ew_game_instance))
        (cast `/Game/Blueprints/Player/BPP_P_Arm` _asbpp_body_part
          (:`then`
            (`KismetSystemLibrary.PrintText` "arm")
            (`PlayerCameraManager.SetManualCameraFade` :`self` (`PlayerController.PlayerCameraManager` (`GameplayStatics.GetPlayerController` 0)) :`InFadeAmount` 1.0))
          (:`CastFailed`
            (cast `/Game/Blueprints/Player/BP_P_LeftLeg` OtherActor
              (:`then`
                (`KismetSystemLibrary.PrintText` "leg")
                (`PlayerCameraManager.SetManualCameraFade` :`self` (`PlayerController.PlayerCameraManager` (`GameplayStatics.GetPlayerController` 0)) :`InFadeAmount` 1.0))
              (:`CastFailed`
                (bind _asbp_p_torso (cast `/Game/Blueprints/Player/BP_P_Torso` OtherActor))
                (if (not (>= (`/Game/Blueprints/Player/BPP_BodyPart.eyeCount` _asbp_p_torso) 1))
                  (`PlayerCameraManager.SetManualCameraFade` :`self` (`PlayerController.PlayerCameraManager` (`GameplayStatics.GetPlayerController` 0)) :`InFadeAmount` 1.0))))))
        (else
          (`PlayerCameraManager.SetManualCameraFade` :`self` (`PlayerController.PlayerCameraManager` (`GameplayStatics.GetPlayerController` 0))))))
    (:`CastFailed`
      (cast `Pawn` OtherActor)
      (`PlayerCameraManager.SetManualCameraFade` :`self` (`PlayerController.PlayerCameraManager` (`GameplayStatics.GetPlayerController` 0))))))

(event `self.Box.OnComponentEndOverlap`
  (params (OverlappedComponent :type "PrimitiveComponent Object Reference") (OtherActor :type "Actor Object Reference") (OtherComp :type "PrimitiveComponent Object Reference") (OtherBodyIndex :type Integer))
  (bind _asbpp_body_part (cast `/Game/Blueprints/Player/BPP_BodyPart` OtherActor))
  (`KismetArrayLibrary.Array_RemoveItem` (`self.MembresAffectés`) _asbpp_body_part)
  (bind _asbp_gi_ew_game_instance (cast `/Game/Blueprints/Managing/BP_GI_EwGameInstance` (`GameplayStatics.GetGameInstance`)))
  (if (not (`KismetArrayLibrary.Array_Contains` (`self.MembresAffectés`) (`/Game/Blueprints/Managing/BP_GI_EwGameInstance.CurrentControlledPart` _asbp_gi_ew_game_instance)))
    (`PlayerCameraManager.SetManualCameraFade` :`self` (`PlayerController.PlayerCameraManager` (`GameplayStatics.GetPlayerController` 0)))))

(fn `CurrentControlledPart`
  (params (CurrentControlledPart :type "/Game/Blueprints/Player/BPP_BodyPart Object Reference")))

(fn `UserConstructionScript`)