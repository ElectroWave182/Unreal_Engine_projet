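; Pipe actor (Tuyau) that teleports player body-part pawns to a linked target pipe, TuyauCible.
; Box overlap identifies a torso, arm or leg and checks that part's entry in the CanGoThrought array.
; If State is true and the target is valid, the pawn moves to the target's location after a short delay.
; The Signal event only prints whether State is open or closed, without changing it.
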(event `/Game/Blueprints/Interactive/Interfaces/BPI_ReceiveSignal.ReceiveSignal`
  (if (`self.state`)
    (`KismetSystemLibrary.PrintString` "Ouvert")
    (else
      (`KismetSystemLibrary.PrintString` "Ferme"))))

(event `self.Box.OnComponentBeginOverlap`
  (params (OverlappedComponent :type "PrimitiveComponent Object Reference") (OtherActor :type "Actor Object Reference") (OtherComp :type "PrimitiveComponent Object Reference") (OtherBodyIndex :type Integer) (bFromSweep :type Boolean) (SweepResult :type "HitResult Structure (by ref)"))
  (bind (_returnvalue_x _returnvalue_y _returnvalue_z) (`KismetMathLibrary.BreakVector` (`self.K2_GetActorLocation` (`self.TuyauCible`))))
  (cast `/Game/Blueprints/Player/BP_P_Torso` OtherActor
    (:`then`
      (if (`|GetArrayItem` (`self.canGoThrought`))
        (if (`self.state`) :!label _label
          (`/Engine/EditorBlueprintResources/StandardMacros.IsValid` (`self.TuyauCible`)
            (:`Is Valid`
              (`KismetSystemLibrary.Delay` 0.5)
              (`self.K2_SetActorLocation` OtherActor (`KismetMathLibrary.MakeVector` _returnvalue_x _returnvalue_y _returnvalue_z) false false))))))
    (:`CastFailed`
      (cast `/Game/Blueprints/Player/BPP_P_Arm` OtherActor
        (:`then`
          (if (`|GetArrayItem` (`self.canGoThrought`) 1)
            (goto _label)))
        (:`CastFailed`
          (cast `/Game/Blueprints/Player/BPP_P_Leg` OtherActor)
          (if (`|GetArrayItem` (`self.canGoThrought`) 2)
            (goto _label)))))))

(fn `UserConstructionScript`)