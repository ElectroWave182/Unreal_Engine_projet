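; Checkpoint actor meant to snapshot puzzle actor states when the player torso passes through, though its overlap logic is disconnected.
; Enregistrer fills per-type maps with activator, lever and receiver states, platform and door rotations, and pushable locations, printing debug text.
; Charger is a TODO stub: its restore logic for replaying those maps is unwired and never applies pushable locations.
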(event `self.ReceiveBeginPlay`
  (`parent.ReceiveBeginPlay`))

(event `self.ReceiveActorBeginOverlap`
  (params (OtherActor :type "Actor Object Reference"))
  ;[0.7083 0.7083 0.7083 0.5] Passage dans le checkpoint
)

(fn `charger`
  (locals (receveur :type "/Game/Blueprints/Interactive/Receiver/BPP_A_Receiver Object Reference"))
  ;[0.15 0 0.001279 0.5] TODO
)

(fn `enregistrer`
  ;[0.4287 0.1845 0.6795 0.502] Interrupteurs : parcourt les états pour les enregistrer un par un, mais pas pour les leviers !
  (`BlueprintMapLibrary.Map_Clear` (`self.sauvegardeInterrupteurs`))
  (bind _outactors (`GameplayStatics.GetAllActorsOfClass` "/Game/Blueprints/Interactive/Trigger/BP_A_Activator.BP_A_Activator_C"))
  (for _array_element _outactors
    (cast `/Game/Blueprints/Interactive/Trigger/BP_A_Lever` _array_element
      (:`CastFailed`
        ;[0.9948 0.03942 0.826 0.5] Debug
        (`KismetSystemLibrary.PrintString` (`KismetStringLibrary.Concat_StrStr` "Enregistré : " (`KismetSystemLibrary.GetDisplayName` _array_element)) true true (struct :`R` 0.300544 :`A` 1.0))
        (`BlueprintMapLibrary.Map_Add` (`self.sauvegardeInterrupteurs`) _array_element (`/Game/Blueprints/Interactive/Trigger/BP_A_Activator.hasBeenTrig` _array_element)))))
  ;[0.4287 0.1845 0.6795 0.502] Leviers : parcourt les états pour les enregistrer un par un
  (`BlueprintMapLibrary.Map_Clear` (`self.sauvegardeLeviers`))
  (bind _outactors_2 (`GameplayStatics.GetAllActorsOfClass` "/Game/Blueprints/Interactive/Trigger/BP_A_Lever.BP_A_Lever_C"))
  (for _array_element_2 _outactors_2
    ;[0.9948 0.03942 0.826 0.5] Debug
    (`KismetSystemLibrary.PrintString` (`KismetStringLibrary.Concat_StrStr` "Enregistré : " (`KismetSystemLibrary.GetDisplayName` _array_element_2)) true true (struct :`R` 0.300544 :`A` 1.0))
    (`BlueprintMapLibrary.Map_Add` (`self.sauvegardeLeviers`) _array_element_2 (`/Game/Blueprints/Interactive/Trigger/BP_A_Activator.hasBeenTrig` _array_element_2)))
  ;[0.05781 0.2582 0.3325 0.502] Receveurs : parcourt les états pour les enregistrer un par un
  (`BlueprintMapLibrary.Map_Clear` (`self.sauvegardeReceveurs`))
  (bind _outactors_3 (`GameplayStatics.GetAllActorsOfClass` "/Game/Blueprints/Interactive/Receiver/BPP_A_Receiver.BPP_A_Receiver_C"))
  (for _array_element_3 _outactors_3
    ;[0.9948 0.03942 0.826 0.5] Debug
    (`KismetSystemLibrary.PrintString` (`KismetStringLibrary.Concat_StrStr` "Enregistré : " (`KismetSystemLibrary.GetDisplayName` _array_element_3)) true true (struct :`R` 0.300544 :`A` 1.0))
    (`BlueprintMapLibrary.Map_Add` (`self.sauvegardeReceveurs`) _array_element_3 (`/Game/Blueprints/Interactive/Receiver/BPP_A_Receiver.state` _array_element_3)))
  ;[0.05781 0.2582 0.3325 0.502] Plateformes rotatives : parcourt les rotations pour les enregistrer une par une
  (`BlueprintMapLibrary.Map_Clear` (`self.sauvegardePlateformesRotatives`))
  (bind _outactors_4 (`GameplayStatics.GetAllActorsOfClass` "/Game/Blueprints/Interactive/Stale/BP_A_RotatingPlatform.BP_A_RotatingPlatform_C"))
  (for _array_element_4 _outactors_4
    ;[0.9948 0.03942 0.826 0.5] Debug
    (`KismetSystemLibrary.PrintString` (`KismetStringLibrary.Concat_StrStr` "Enregistré : " (`KismetSystemLibrary.GetDisplayName` _array_element_4)) true true (struct :`R` 0.351533 :`G` 0.456411 :`B` 1.0 :`A` 1.0))
    (`BlueprintMapLibrary.Map_Add` (`self.sauvegardePlateformesRotatives`) _array_element_4 (`/Game/Blueprints/Interactive/Stale/BP_A_RotatingPlatform.Rotation` _array_element_4)))
  ;[0.15 0.1441 0.1119 0.502] Portes physiques : parcourt les rotations pour les enregistrer une par une
  (`BlueprintMapLibrary.Map_Clear` (`self.sauvegardePortePhysique`))
  (bind _outactors_5 (`GameplayStatics.GetAllActorsOfClass` "/Game/Blueprints/Interactive/Physical/BP_A_PhysicsDoor.BP_A_PhysicsDoor_C"))
  (for _array_element_5 _outactors_5
    ;[0.9948 0.03942 0.826 0.5] Debug
    (`KismetSystemLibrary.PrintString` (`KismetStringLibrary.Concat_StrStr` "Enregistré : " (`KismetSystemLibrary.GetDisplayName` _array_element_5)) true true (struct :`R` 0.287441 :`G` 0.376262 :`B` 0.814847 :`A` 1.0))
    (`BlueprintMapLibrary.Map_Add` (`self.sauvegardePortePhysique`) _array_element_5 (`SceneComponent.K2_GetComponentRotation` (`/Game/Blueprints/Interactive/Physical/BP_A_PhysicsDoor.Door` _array_element_5))))
  ;[0.15 0.1441 0.1119 0.502] Objets poussables : parcourt les positions pour les enregistrer une par une
  (`BlueprintMapLibrary.Map_Clear` (`self.sauvegardePoussables`))
  (bind _outactors_6 (`GameplayStatics.GetAllActorsOfClass` "/Game/Blueprints/Interactive/Physical/BP_A_Pushable.BP_A_Pushable_C"))
  (for _array_element_6 _outactors_6
    ;[0.9948 0.03942 0.826 0.5] Debug
    (`KismetSystemLibrary.PrintString` (`KismetStringLibrary.Concat_StrStr` "Enregistré : " (`KismetSystemLibrary.GetDisplayName` _array_element_6)) true true (struct :`R` 1.0 :`G` 0.590619 :`B` 0.016807 :`A` 1.0))
    (`BlueprintMapLibrary.Map_Add` (`self.sauvegardePoussables`) _array_element_6 (`self.K2_GetActorLocation` _array_element_6))))

(fn `UserConstructionScript`
  (`parent.UserConstructionScript`))