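; Instrument pickup actor that appears if the game instance's InstrumentMap flags its type, and hands off to an NPC when signaled.
; The construction script picks the mesh from InstrumentStatus.
; Signal reveals it and runs a timeline that spins and shrinks it.
; On finish, Contrebasse and Saxophone start the Mare and Lion NPCs' playing animations respectively, then destroy the actor; an older NPC-search branch sits unconnected.
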(event `self.ReceiveBeginPlay`
  (bind _asbp_gi_ew_game_instance (cast `/Game/Blueprints/Managing/BP_GI_EwGameInstance` (`GameplayStatics.GetGameInstance`)))
  (if (`BlueprintMapLibrary.Map_Find` (`/Game/Blueprints/Managing/BP_GI_EwGameInstance.Instrument Map` _asbp_gi_ew_game_instance) (`self.Instrument Status`))
    (`SceneComponent.SetVisibility` (`self.StaticMesh`) true false)
    (`PrimitiveComponent.SetCollisionEnabled` (`self.StaticMesh`) "QueryAndPhysics")))

(event `/Game/Blueprints/Interactive/Interfaces/BPI_ReceiveSignal.ReceiveSignal`
  (`SceneComponent.SetVisibility` (`self.StaticMesh`) true (`self.baguette`))
  (bind (_direction _animate) (`Timeline|Chronologie` :!via `PlayFromStart`)
    (:`Update`
      (set `RotatingMovementComponent.RotationRate` (`KismetMathLibrary.MakeRotator` 0.0 0.0 (* (+ (* 50.0 _animate) 1.0) 80.0)) (`self.RotatingMovement`))
      (`self.SetActorScale3D` (- 1.0 _animate))
      (`PrimitiveComponent.SetCollisionEnabled` (`self.StaticMesh`) "QueryAndPhysics"))
    (:`Finished`
      (set `RotatingMovementComponent.RotationRate` (struct) (`self.RotatingMovement`))
      (switch `/Game/Utilities/E_InstrumentList` (`self.Instrument Status`)
        (:`NewEnumerator0`
          (bind _returnvalue (`GameplayStatics.GetActorOfClass` "/Game/Blueprints/NPC/SnailandMare/BP_NPC_Mare.BP_NPC_Mare_C"))
          (`KismetSystemLibrary.Delay` 0.7)
          (`/Game/Blueprints/NPC/SnailandMare/BP_NPC_Mare.StartPlayingAnim` _returnvalue)
          (`self.K2_DestroyActor`))
        (:`NewEnumerator3`
          (bind _returnvalue_2 (`GameplayStatics.GetActorOfClass` "/Game/Blueprints/NPC/Lion/BP_NPC_Lion.BP_NPC_Lion_C"))
          (`KismetSystemLibrary.Delay` 0.7)
          (`/Game/Blueprints/NPC/Lion/BP_NPC_Lion.StartPlayingAnim` _returnvalue_2)
          (`self.K2_DestroyActor`))))))

(fn `UserConstructionScript`
  (`parent.UserConstructionScript`)
  (switch `/Game/Utilities/E_InstrumentList` (`self.Instrument Status`)
    (:`NewEnumerator0`
      (`StaticMeshComponent.SetStaticMesh` (`self.StaticMesh`) "/Game/Assets/Meshes/Lounge/SM_Contrebasse.SM_Contrebasse"))
    (:`NewEnumerator1`
      (`StaticMeshComponent.SetStaticMesh` (`self.StaticMesh`) "/Game/Assets/Meshes/Lounge/SM_Timbale.SM_Timbale"))
    (:`NewEnumerator2`
      (`StaticMeshComponent.SetStaticMesh` (`self.StaticMesh`) "/Game/Assets/Meshes/Lounge/SM_Tuba.SM_Tuba"))
    (:`NewEnumerator3`
      (`StaticMeshComponent.SetStaticMesh` (`self.StaticMesh`) "/Game/Assets/Meshes/Lounge/SM_Saxophone.SM_Saxophone"))
    (:`NewEnumerator4`
      (`StaticMeshComponent.SetStaticMesh` (`self.StaticMesh`) "/Game/Assets/Meshes/Lounge/SM_Synthetizer.SM_Synthetizer"))))