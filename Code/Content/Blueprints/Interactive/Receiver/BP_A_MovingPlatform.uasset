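; Signal-driven moving platform that travels through waypoints built from chained relative MoveToPose offsets, in One Shot, One Shot Reverse or Ping Pong mode.
; A timeline lerps location and rotation per segment, its play rate scaled by distance for constant speed, with waits at turnarounds.
; Deactivation sends it back toward the start.
; The construction script draws the path and applies the colour material, whose emission reflects the active state.
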(event `self.ReceiveBeginPlay`
  (bind _destinationtransform (`self.DestinationTransform`))
  ; Initialisation
  (`self.InitGameInstance`)
  (bind _output_get (set `self.CacheTransform` (`self.GetTransform`)))
  (`KismetArrayLibrary.Array_Add` _destinationtransform _output_get)
  (for _array_element (`self.moveToPose`)
    (bind _output_get_2 (set `self.CacheTransform` (`KismetMathLibrary.MakeTransform` (+ (.location _array_element) (.location _output_get)) (.rotation _array_element) (.scale _output_get))))
    (`KismetArrayLibrary.Array_Add` _destinationtransform _output_get_2))
  ;; Set Material Instance
  (bind _returnvalue (`PrimitiveComponent.CreateDynamicMaterialInstance` (`self.StaticMesh`) 0 (`self.materialToApply`) "None"))
  (bind _output_get_3 (set `self.materialInstance` _returnvalue))
  (bind _returnvalue_2 (`MaterialInstanceDynamic.K2_GetScalarParameterValue` _output_get_3 "EmissionStrength"))
  (set `self.emissionStrength` _returnvalue_2)
  (`MaterialInstanceDynamic.SetScalarParameterValue` _output_get_3 "EmissionStrength" 1.0)
  (if (`self.state`)
    (`self.SwitchTree`)
    (`MaterialInstanceDynamic.SetScalarParameterValue` (`self.materialInstance`) "EmissionStrength" (`self.emissionStrength`))))

(event `/Game/Blueprints/Interactive/Interfaces/BPI_ReceiveSignal.ReceiveSignal`
  (bind _materialinstance (`self.materialInstance`))
  ; Switch between states
  (if (`self.state`)
    (`self.PlaySFX` "NewEnumerator0")
    (set `self.isInversed` false)
    (set `self.DestinationIndex` 0)
    (`self.SwitchTree`)
    ; Emissive when activated
    (`MaterialInstanceDynamic.SetScalarParameterValue` _materialinstance "EmissionStrength" (`self.emissionStrength`))
    (else
      (`self.PlaySFX` "NewEnumerator1")
      (`self.StopAnimate`)
      (`MaterialInstanceDynamic.SetScalarParameterValue` _materialinstance "EmissionStrength" 1.0))))

(event `SwitchTree`
  ; Switch tree of behaviour
  (switch `/Game/Utilities/EMovingBehaviour` (`self.Behaviour Type`)
    (:`NewEnumerator0`
      (`KismetSystemLibrary.PrintText` "Behaviour not assigned"))
    (:`NewEnumerator1`
      (`self.StartAnimate` :!label _label))
    (:`NewEnumerator2`
      (set `self.Will Inverse` true)
      (goto _label))
    (:`NewEnumerator3`
      (set `self.Will Ping Pong` true)
      (goto _label))))

(event `StartAnimate`
  (bind (_cachetransform_location _cachetransform_rotation _cachetransform_scale) (`KismetMathLibrary.BreakTransform` (`self.CacheTransform`)))
  (bind _destinationindex (`self.DestinationIndex`))
  (bind _destinationindex_2 (`self.DestinationIndex`))
  (if (`self.isInversed`) :!label _label_2
    (`/Engine/EditorBlueprintResources/StandardMacros.DecrementInt` _destinationindex_2 :!label _label_3
      (:`  `
        _))
    (else
      (`/Engine/EditorBlueprintResources/StandardMacros.IncrementInt` _destinationindex_2
        (:`  `
          _))))
  (set `self.CacheTransform` (`self.GetTransform`) :!label _label_4)
  (`self.UpdateSpeed`)
  (bind (_direction _alpha) (`Timeline|Timeline` :!via `PlayFromStart`)
    (:`Update`
      ; Platform Movement
      (`self.K2_SetActorTransform` (`KismetMathLibrary.MakeTransform` (`KismetMathLibrary.VLerp` _cachetransform_location (.location (`|GetArrayItem` (`self.DestinationTransform`) (`self.DestinationIndex`))) _alpha) (`KismetMathLibrary.RLerp` _cachetransform_rotation (.rotation (`|GetArrayItem` (`self.DestinationTransform`) (`self.DestinationIndex`))) _alpha) _cachetransform_scale)))
    (:`Finished`
      (if (and (< _destinationindex (- (`KismetArrayLibrary.Array_Length` (`self.DestinationTransform`)) 1)) (> _destinationindex 0))
        (`self.StartAnimate`)
        (else
          ; OneShotReverse logic
          (if (`self.Will Inverse`)
            (set `self.isInversed` true)
            (set `self.Will Inverse` false)
            (if (`self.state`) :!label _label_5
              (if (`self.hasBeenDeactivated`)
                (set `self.hasBeenDeactivated` false))
              (`KismetSystemLibrary.RetriggerableDelay` (`self.WaitingTime`))
              (if (not (`self.hasBeenDeactivated`))
                (`self.StartAnimate`)))
            (else
              ; PingPong logic
              (if (`self.Will Ping Pong`)
                (if (`self.isInversed`)
                  (set `self.isInversed` false)
                  (goto _label_5)
                  (else
                    (set `self.isInversed` true)
                    (goto _label_5)))))))))))

(event `StopAnimate`
  (set `self.hasBeenDeactivated` true)
  (set `self.Will Inverse` false)
  (set `self.Will Ping Pong` false)
  (if (not (`self.isInversed`))
    (if (not (== (`self.DestinationIndex`) 0))
      (set `self.isInversed` true)
      (goto _label_2))
    (elif (== (`self.DestinationIndex`) (- (`KismetArrayLibrary.Array_Length` (`self.DestinationTransform`)) 1))
      (goto _label_3)
      (else
        (goto _label_4)))))

(fn `ApplyMaterialColor`
  (`PrimitiveComponent.SetMaterial` (`self.StaticMesh`) 0 (`self.materialToApply`)))

(fn `SaveMaterialColor`
  (switch `/Game/Utilities/EMaterialColor` (`self.materialColor`)
    (:`NewEnumerator0`
      (set `self.materialToApply` "/Game/Assets/Materials/Material_Puzzle/Materiaux_Triggers/MI_Triggers_Blanc.MI_Triggers_Blanc"))
    (:`NewEnumerator1`
      (set `self.materialToApply` "/Game/Assets/Materials/Material_Puzzle/Materiaux_Triggers/MI_Triggers_Bleu.MI_Triggers_Bleu"))
    (:`NewEnumerator2`
      (set `self.materialToApply` "/Game/Assets/Materials/Material_Puzzle/Materiaux_Triggers/MI_Triggers_Orange.MI_Triggers_Orange"))
    (:`NewEnumerator3`
      (set `self.materialToApply` "/Game/Assets/Materials/Material_Puzzle/Materiaux_Triggers/MI_Triggers_Rose.MI_Triggers_Rose"))
    (:`NewEnumerator4`
      (set `self.materialToApply` "/Game/Assets/Materials/Material_Puzzle/Materiaux_Triggers/MI_Triggers_Rouge.MI_Triggers_Rouge"))
    (:`NewEnumerator5`
      (set `self.materialToApply` "/Game/Assets/Materials/Material_Puzzle/Materiaux_Triggers/MI_Triggers_Vert.MI_Triggers_Vert"))))

(fn `UpdateSpeed`
  ; Update speed
  (`TimelineComponent.SetPlayRate` (`self.Timeline`) (/ (`self.Speed`) (`KismetMathLibrary.VSize` (- (`self.K2_GetActorLocation`) (.location (`|GetArrayItem` (`self.DestinationTransform`) (`self.DestinationIndex`))))))))

(fn `UserConstructionScript`
  (locals (LastPos :type "Vector Structure"))
  (bind _lastpos (`local.LastPos`))
  ; Draw MoveToPose positions
  (set `local.LastPos` (`self.K2_GetActorLocation`))
  (for _array_element (`self.moveToPose`)
    (bind _returnvalue (+ (.location _array_element) _lastpos))
    (`KismetSystemLibrary.DrawDebugArrow` _lastpos _returnvalue 5.0 (struct) 5.0 5.0)
    (set `local.LastPos` _returnvalue)
    ; Apply Color
    (`self.SaveMaterialColor`)
    (`self.ApplyMaterialColor`)))