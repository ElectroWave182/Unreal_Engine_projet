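; A receiver door that slides vertically open or closed when signaled, according to its State, and starts opening at BeginPlay if State is already true.
; A timeline lerps the door's relative Z, with play rate derived from separate open and close durations.
; A dynamic material raises emission to its authored strength when active and resets it otherwise, while signals also play sounds.
; Outside the lounge variant, the construction script applies the selected color material.
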(event `self.ReceiveBeginPlay`
  (`self.InitGameInstance`)
  ; Set Material Instance
  (bind _returnvalue (`PrimitiveComponent.CreateDynamicMaterialInstance` (`self.door`) 0 (`self.Material to Apply`) "None"))
  (bind _output_get (set `self.materialInstance` _returnvalue))
  (bind _returnvalue_2 (`MaterialInstanceDynamic.K2_GetScalarParameterValue` _output_get "EmissionStrength"))
  (set `self.emissionStrength` _returnvalue_2)
  (`MaterialInstanceDynamic.SetScalarParameterValue` _output_get "EmissionStrength" 1.0)
  (if (`self.state`)
    (`MaterialInstanceDynamic.SetScalarParameterValue` (`self.materialInstance`) "EmissionStrength" (`self.emissionStrength`) :!label _label)
    (`self.SetSpeed` (`self.secondsToOpen`))
    (bind (_direction _opennig_door) (`Timeline|Door Timeline` :!label _label_2)
      (:`Update`
        (`SceneComponent.K2_SetRelativeLocation` (`self.door`) (`KismetMathLibrary.MakeVector` 0.0 0.0 (`KismetMathLibrary.Lerp` 0.0 (`self.ZDifference`) _opennig_door)) false false)))))

(event `/Game/Blueprints/Interactive/Interfaces/BPI_ReceiveSignal.ReceiveSignal`
  (if (`self.state`)
    (`self.PlaySFX` "NewEnumerator15")
    (goto _label)
    (else
      (`self.PlaySFX` "NewEnumerator16")
      (`MaterialInstanceDynamic.SetScalarParameterValue` (`self.materialInstance`) "EmissionStrength" 1.0)
      (`self.SetSpeed` (`self.secondsToClose`))
      (goto _label_2 :!via `Reverse`))))

(fn `ApplyMaterialColor`
  (`PrimitiveComponent.SetMaterial` (`self.door`) 0 (`self.Material to Apply`)))

(fn `SaveMaterialColor`
  (switch `/Game/Utilities/EMaterialColor` (`self.Material Color`)
    (:`NewEnumerator0`
      (set `self.Material to Apply` "/Game/Assets/Materials/Material_Puzzle/Materiaux_Triggers/MI_Triggers_Blanc.MI_Triggers_Blanc"))
    (:`NewEnumerator1`
      (set `self.Material to Apply` "/Game/Assets/Materials/Material_Puzzle/Materiaux_Triggers/MI_Triggers_Bleu.MI_Triggers_Bleu"))
    (:`NewEnumerator2`
      (set `self.Material to Apply` "/Game/Assets/Materials/Material_Puzzle/Materiaux_Triggers/MI_Triggers_Orange.MI_Triggers_Orange"))
    (:`NewEnumerator3`
      (set `self.Material to Apply` "/Game/Assets/Materials/Material_Puzzle/Materiaux_Triggers/MI_Triggers_Rose.MI_Triggers_Rose"))
    (:`NewEnumerator4`
      (set `self.Material to Apply` "/Game/Assets/Materials/Material_Puzzle/Materiaux_Triggers/MI_Triggers_Rouge.MI_Triggers_Rouge"))
    (:`NewEnumerator5`
      (set `self.Material to Apply` "/Game/Assets/Materials/Material_Puzzle/Materiaux_Triggers/MI_Triggers_Vert.MI_Triggers_Vert"))))

(fn `SetSpeed`
  (params (newSpeed :type "Float (double-precision)"))
  (`TimelineComponent.SetPlayRate` (`self.Door Timeline`) (/ 1.0 newSpeed)))

(fn `UserConstructionScript`
  (if (not (`self.IsLounge`))
    (`self.SaveMaterialColor`)
    (`self.ApplyMaterialColor`)))