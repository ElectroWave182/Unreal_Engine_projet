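; Lever trigger that the player interacts with to toggle the state of its linked receivers.
; An interact check validates pawn conditions, plays a sound, then plays or reverses a timeline that rotates the animated part, depending on the current triggered state.
; When the timeline finishes, it calls the camera switch, changes each receiver's state and flips the triggered flag.
; Body part overlaps toggle or reset the interaction UI.
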(event `self.ReceiveBeginPlay`
  (`self.InitGameInstance`))

(event `/Game/Blueprints/Interactive/Interfaces/BPI_InteractionSignal.InteractCheck`
  ; Receiving Check on IA_Interact
  (bind _isvalid (`self.CheckPawnConditions`))
  (if _isvalid
    (if (`self.hasBeenTrig`)
      (`self.PlaySFX` "NewEnumerator12")
      ; Lever Animation
      (bind (_direction _nouvelle_piste_0) (`Timeline|Plate Timeline_0` :!via `Reverse` :!label _label)
        (:`Update`
          (`SceneComponent.K2_SetRelativeRotation` (`self.AnimatedPart`) (`KismetMathLibrary.MakeRotator` (`KismetMathLibrary.Lerp` 45.0 135.0 _nouvelle_piste_0)) false false))
        (:`Finished`
          (`self.SwitchToCamera`)
          (for _array_element (`self.Receivers`)
            (`/Game/Blueprints/Interactive/Interfaces/BPI_SignalsToReceiver.ChangeReceiverState` _array_element))
          (set `self.hasBeenTrig` (not (`self.hasBeenTrig`)))))
      (else
        (`self.PlaySFX` "NewEnumerator10")
        (goto _label)))))

(event `self.ReceiveActorBeginOverlap`
  (params (OtherActor :type "Actor Object Reference"))
  ; Overlapping bodypart --> UI change
  (cast `/Game/Blueprints/Player/BPP_BodyPart` OtherActor)
  (`self.UITriggerToggle` "NewEnumerator6"))

(event `self.ReceiveActorEndOverlap`
  (params (OtherActor :type "Actor Object Reference"))
  ; Overlapping bodypart --> UI change
  (cast `/Game/Blueprints/Player/BPP_BodyPart` OtherActor)
  (`self.ResetUIIfnecessary`))

(fn `UserConstructionScript`)