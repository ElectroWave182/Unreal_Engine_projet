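; Trigger actor that switches one player power on or off, depending on its configured PowerState, when a BPP_BodyPart overlaps it.
; A looping timeline spins the Power component around yaw as an idle animation.
; If the power's state in BP_PlayerManager's PowerStates map needs changing, it plays a sound, updates the map, notifies the manager and refreshes the main HUD.
; It then stops the spin and hides the Power component.
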(event `self.ReceiveBeginPlay`
  ; Animation
  (`self.InitGameInstance`)
  (bind (_direction _alpha) (`Timeline|HandAnimation` :!via `PlayFromStart` :!label _label)
    (:`Update`
      (`SceneComponent.K2_SetRelativeRotation` (`self.Power`) (`KismetMathLibrary.MakeRotator` 0.0 0.0 (`KismetMathLibrary.Lerp` 0.0 360.0 _alpha)) false false))
    (:`Finished`
      (goto _label :!via `PlayFromStart`))))

(event `StopAnimation`
  ; Animation
  (goto _label :!via `Stop`))

(event `self.ReceiveActorBeginOverlap`
  (params (OtherActor :type "Actor Object Reference"))
  (bind _returnvalue (`|GetEnumeratorNameAsString` (`self.PowerType`)))
  (bind _returnvalue_2 (`|GetEnumeratorNameAsString` (`self.PowerType`)))
  (cast `/Game/Blueprints/Player/BPP_BodyPart` OtherActor)
  (bind _returnvalue_3 (`GameplayStatics.GetActorOfClass` "/Game/Blueprints/Managing/BP_PlayerManager.BP_PlayerManager_C"))
  (switch `/Game/Utilities/EPowerState` (`self.PowerState`)
    (:`NewEnumerator0`
      (bind _powerstates (`/Game/Blueprints/Managing/BP_PlayerManager.powerStates` _returnvalue_3))
      (if (not (`BlueprintMapLibrary.Map_Find` _powerstates _returnvalue_2))
        (`self.PlayTogglerSFX` "NewEnumerator10")
        (`BlueprintMapLibrary.Map_Add` _powerstates _returnvalue_2 true)
        (`/Game/Blueprints/Managing/BP_PlayerManager.ChangePowerEnabledFromManager` _returnvalue_3 :!label _label_2)
        (`self.Update MainHUD`)
        ; Animation
        (`self.StopAnimation`)
        (`SceneComponent.SetVisibility` (`self.Power`) false false)))
    (:`NewEnumerator1`
      (bind _powerstates_2 (`/Game/Blueprints/Managing/BP_PlayerManager.powerStates` _returnvalue_3))
      (if (`BlueprintMapLibrary.Map_Find` _powerstates_2 _returnvalue)
        (`self.PlayTogglerSFX` "NewEnumerator11")
        (`BlueprintMapLibrary.Map_Add` _powerstates_2 _returnvalue)
        (goto _label_2)))))

(fn `InitGameInstance`
  (bind _asbp_gi_ew_game_instance (cast `/Game/Blueprints/Managing/BP_GI_EwGameInstance` (`GameplayStatics.GetGameInstance`)))
  (set `self.Game Instance` _asbp_gi_ew_game_instance))

(fn `PlayTogglerSFX`
  (params (Type :type "/Game/Utilities/ESFX_Global Enum" :default "NewEnumerator0"))
  (`/Game/Blueprints/Managing/BP_GI_EwGameInstance.Play2DSound` (`self.Game Instance`) self Type))

(fn `Update MainHUD`
  (bind _asbp_ewhud (cast `/Game/Blueprints/Managing/BP_EWHUD` (`PlayerController.GetHUD` (`GameplayStatics.GetPlayerController` 0))))
  (bind _ref_mainhud (`/Game/Blueprints/Managing/BP_EWHUD.Ref_MainHUD` _asbp_ewhud))
  (`/Game/Blueprints/UI/HUD/WBP_MainHUD.SwitchVisibilityHUD` _ref_mainhud (`/Game/Blueprints/UI/HUD/WBP_MainHUD.Current Selected` _ref_mainhud)))

(fn `UserConstructionScript`)