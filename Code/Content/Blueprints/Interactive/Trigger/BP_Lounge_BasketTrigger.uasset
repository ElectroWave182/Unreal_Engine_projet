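; BP_Lounge_BasketTrigger is a Lounge trigger that reveals a hidden instrument when a BPP_P_Arm actor overlaps it.
; BeginPlay hides the referenced Instrument's mesh and disables its box collision.
; The overlap restores both, plays a sound at the instrument, destroys a referenced button, then toggles each receiver's state and sets a GameInstance dialogue condition inside that loop.
; The construction script adds relative InterpToMovement control points from origin to ToPosition.
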(event `self.ReceiveBeginPlay`
  (`self.InitGameInstance`)
  (`SceneComponent.SetVisibility` (`/Game/Blueprints/Interactive/Trigger/BPP_A_Instrument.StaticMesh` (`self.Instrument`)) false false)
  (`PrimitiveComponent.SetCollisionEnabled` (`/Game/Blueprints/Interactive/Trigger/BPP_A_Instrument.Box` (`self.Instrument`)) "NoCollision"))

(event `self.  dddd.OnComponentBeginOverlap`
  (params (OverlappedComponent :type "PrimitiveComponent Object Reference") (OtherActor :type "Actor Object Reference") (OtherComp :type "PrimitiveComponent Object Reference") (OtherBodyIndex :type Integer) (bFromSweep :type Boolean) (SweepResult :type "HitResult Structure (by ref)"))
  (bind _instrument (`self.Instrument`))
  (if (`KismetMathLibrary.ClassIsChildOf` (`GameplayStatics.GetObjectClass` OtherActor) "/Game/Blueprints/Player/BPP_P_Arm.BPP_P_Arm_C")
    (`SceneComponent.SetVisibility` (`/Game/Blueprints/Interactive/Trigger/BPP_A_Instrument.StaticMesh` _instrument) true false)
    (`PrimitiveComponent.SetCollisionEnabled` (`/Game/Blueprints/Interactive/Trigger/BPP_A_Instrument.Box` (`self.Instrument`)) "QueryAndPhysics")
    ;[0.009866 0 0.15 0.5] TODO - NANA - SFX Type Should depend on the instrument ?
    (`self.PlaySFXAtAnotherLocation` "NewEnumerator0" _instrument)
    (`self.K2_DestroyActor` (`self.BUTTON TO DESTROY`))
    (for _array_element (`self.Receivers`)
      (`self.ChangeReceiverState` _array_element)
      (bind _asbp_gi_ew_game_instance (cast `/Game/Blueprints/Managing/BP_GI_EwGameInstance` (`GameplayStatics.GetGameInstance`)))
      (`KismetArrayLibrary.Array_Set` (`/Game/Blueprints/Managing/BP_GI_EwGameInstance.DialogueConditions` _asbp_gi_ew_game_instance) 11 true))))

(fn `UserConstructionScript`
  (`InterpToMovementComponent.AddControlPointPosition` (`self.InterpToMovement`) (0.0 0.0 0.0) true)
  (`InterpToMovementComponent.AddControlPointPosition` (`self.InterpToMovement`) (`self.ToPosition`) true))