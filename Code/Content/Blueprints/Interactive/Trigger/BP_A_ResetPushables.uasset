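; Pressure plate trigger that returns a list of pushable objects to their initial transforms.
; Overlapping its collision plays a sound and a Timeline that lowers the plate and changes its emission through a dynamic material instance.
; When the press animation finishes, each pushable is moved back and its linear velocity zeroed.
; Ending the overlap plays a sound and reverses the Timeline, with HasBeenTrig preventing a reset on release.
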(event `self.ReceiveBeginPlay`
  (bind _animatedpart (`self.AnimatedPart`))
  ; Set Material Instance
  (`self.InitGameInstance`)
  (bind _returnvalue (`PrimitiveComponent.CreateDynamicMaterialInstance` _animatedpart 0 (`PrimitiveComponent.GetMaterial` _animatedpart 0) "None"))
  (bind _output_get (set `self.materialInstance` _returnvalue))
  (bind _returnvalue_2 (`MaterialInstanceDynamic.K2_GetScalarParameterValue` _output_get "EmissionStrength"))
  (set `self.emissionStrength` _returnvalue_2))

(event `self.Collision.OnComponentBeginOverlap`
  (params (OverlappedComponent :type "PrimitiveComponent Object Reference") (OtherActor :type "Actor Object Reference") (OtherComp :type "PrimitiveComponent Object Reference") (OtherBodyIndex :type Integer) (bFromSweep :type Boolean) (SweepResult :type "HitResult Structure (by ref)"))
  (if (not (`self.hasBeenTrig`))
    (set `self.hasBeenTrig` true)
    (`self.PlaySFX` "NewEnumerator2")
    ; Plate Animation
    (bind (_direction _nouvelle_piste_0) (`Timeline|Timeline` :!label _label)
      (:`Update`
        (`SceneComponent.K2_SetRelativeLocation` (`self.AnimatedPart`) (`KismetMathLibrary.MakeVector` 0.0 0.0 (`KismetMathLibrary.Lerp` 10.0 1.0 _nouvelle_piste_0)) false false)
        (`MaterialInstanceDynamic.SetScalarParameterValue` (`self.materialInstance`) "EmissionStrength" (`KismetMathLibrary.Lerp` (`self.emissionStrength`) 10.0 _nouvelle_piste_0)))
      (:`Finished`
        (if (`self.hasBeenTrig`)
          (for _array_element (`self.pushablesToReset`)
            (`self.K2_SetActorTransform` _array_element (`/Game/Blueprints/Interactive/Physical/BP_A_Pushable.InitialTransform` _array_element) false false)
            (`PrimitiveComponent.SetPhysicsLinearVelocity` (`/Game/Blueprints/Interactive/Physical/BP_A_Pushable.BoxSkin` _array_element) (0.0 0.0 0.0) false "None")))))))

(event `self.Collision.OnComponentEndOverlap`
  (params (OverlappedComponent :type "PrimitiveComponent Object Reference") (OtherActor :type "Actor Object Reference") (OtherComp :type "PrimitiveComponent Object Reference") (OtherBodyIndex :type Integer))
  (if (`self.hasBeenTrig`)
    (set `self.hasBeenTrig` false)
    (`self.PlaySFX` "NewEnumerator3")
    (goto _label :!via `Reverse`)))

(fn `InitGameInstance`
  (bind _asbp_gi_ew_game_instance (cast `/Game/Blueprints/Managing/BP_GI_EwGameInstance` (`GameplayStatics.GetGameInstance`)))
  (set `self.Game Instance` _asbp_gi_ew_game_instance))

(fn `PlaySFX`
  (params (Type :type "/Game/Utilities/ESFX_Enviro Enum" :default "NewEnumerator0"))
  (`/Game/Blueprints/Managing/BP_GI_EwGameInstance.PlayInteractiveSound` (`self.Game Instance`) self Type))

(fn `UserConstructionScript`)