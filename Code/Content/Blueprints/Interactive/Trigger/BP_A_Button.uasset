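; Single-use interactive button that changes the state of its linked receivers when an interaction passes the pawn condition check.
; A timeline slides the animated part in, then sets the dynamic material's emission, updates the receivers and calls a camera switch.
; Body-part overlaps toggle the trigger UI until the button is used.
; ResetSignal changes receivers again if triggered, clears the used flag and rewinds the timeline.
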(event `self.ReceiveBeginPlay`
  ; Set Material Instance
  (`self.InitGameInstance`)
  (bind _returnvalue (`PrimitiveComponent.CreateDynamicMaterialInstance` (`self.AnimatedPart`) 0 (`self.materialToApply`) "None"))
  (set `self.materialInstance` _returnvalue))

(event `/Game/Blueprints/Interactive/Interfaces/BPI_InteractionSignal.InteractCheck`
  ; Receiving Check on IA_Interact conditionned by Has Been Trig (single time trig)
  (bind _isvalid (`self.CheckPawnConditions`))
  (if _isvalid
    (if (not (`self.hasBeenTrig`))
      (`self.PlaySFX` "NewEnumerator11")
      ; Plate Animation
      (bind (_direction _nouvelle_piste_0) (`Timeline|Timeline` :`NewTime` (`KismetMathLibrary.Conv_BoolToDouble` (`self.hasBeenTrig`)) :!label _label)
        (:`Update`
          (`SceneComponent.K2_SetRelativeLocation` (`self.AnimatedPart`) (`KismetMathLibrary.MakeVector` 0.0 (`KismetMathLibrary.Lerp` 5.0 1.0 _nouvelle_piste_0)) false false))
        (:`Finished`
          ; Button deactivated
          (`MaterialInstanceDynamic.SetScalarParameterValue` (`self.materialInstance`) "EmissionStrength" 1.0)
          (for _array_element (`self.Receivers`)
            (`/Game/Blueprints/Interactive/Interfaces/BPI_SignalsToReceiver.ChangeReceiverState` _array_element))
          (set `self.hasBeenTrig` true)
          (`self.SwitchToCamera`)
          (`self.ResetUIIfnecessary`))))))

(event `/Game/Blueprints/Interactive/Interfaces/BPI_ReceiveSignalsAsTrigger.ReceiveResetSignal`
  ;[0.6667 0.6667 0.6667 0.5] Restore to the initial state
  (if (`self.hasBeenTrig`)
    (for _array_element (`self.Receivers`)
      (`/Game/Blueprints/Interactive/Interfaces/BPI_SignalsToReceiver.ChangeReceiverState` _array_element)))
  (set `self.hasBeenTrig` false)
  (`self.PlaySFX` "NewEnumerator13")
  ; Plate Animation
  (`|ExecutionSequence`
    (:`then_0`
      (goto _label :!via `Stop`))
    (:`then_1`
      (goto _label :!via `SetNewTime`))))

(event `self.ReceiveActorBeginOverlap`
  (params (OtherActor :type "Actor Object Reference"))
  ; Overlapping bodypart --> UI change
  (if (not (`self.hasBeenTrig`))
    (cast `/Game/Blueprints/Player/BPP_BodyPart` OtherActor)
    (`self.UITriggerToggle` "NewEnumerator6")))

(event `self.ReceiveActorEndOverlap`
  (params (OtherActor :type "Actor Object Reference"))
  ; Overlapping bodypart --> UI change
  (if (not (`self.hasBeenTrig`))
    (cast `/Game/Blueprints/Player/BPP_BodyPart` OtherActor)
    (`self.ResetUIIfnecessary`)))

(fn `UserConstructionScript`)