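; Interactive toilet whose seat toggles up and down on interaction, with an optional alien that scales in when the seat is triggered.
; A timeline lerps the seat's roll and, on alien variants, drives a second timeline that scales the alien mesh and disables further interaction.
; Non-alien variants destroy the alien mesh on BeginPlay.
; Body part overlaps toggle the interaction UI; the alien spin logic is disconnected.
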(event `self.ReceiveBeginPlay`
  (`self.InitGameInstance`)
  (if (not (`self.IsAlien`))
    (`ActorComponent.K2_DestroyComponent` (`self.SM_Alien`))))

(event `/Game/Blueprints/Interactive/Interfaces/BPI_InteractionSignal.InteractCheck`
  (if (`self.NotInteractable`)
    _
    (elif (`self.hasBeenTrig`)
      (set `self.hasBeenTrig` false)
      (bind (_direction _rotation) (`Timeline|RotationCuvette` :!via `Reverse` :!label _label)
        (:`Update`
          (`SceneComponent.K2_SetRelativeRotation` (`self.Lunette`) (`KismetMathLibrary.MakeRotator` (`KismetMathLibrary.Lerp` 0.0 (`self.ZDifference`) _rotation)) false false)
          (if (`self.IsAlien`)
            (if (`self.hasBeenTrig`)
              (bind (_direction_2 _alien_rotation _alien_scale) (`Timeline|Timeline` :!via `PlayFromStart` :!label _label_2)
                (:`Update`
                  (`SceneComponent.SetWorldScale3D` (`self.SM_Alien`) _alien_scale)
                  (set `self.NotInteractable` true)))
              (else
                (goto _label_2 :!via `Reverse`))))))
      (else
        (set `self.hasBeenTrig` true)
        (goto _label)))))

(event `self.ReceiveActorBeginOverlap`
  (params (OtherActor :type "Actor Object Reference"))
  ; Overlapping bodypart --> UI change
  (cast `/Game/Blueprints/Player/BPP_BodyPart` OtherActor)
  (`self.UITriggerToggle` "NewEnumerator6"))

(event `self.ReceiveActorEndOverlap`
  (params (OtherActor :type "Actor Object Reference"))
  ; Overlapping bodypart --> UI change
  (cast `/Game/Blueprints/Player/BPP_BodyPart` OtherActor)
  (`self.ResetUIIfnecessary`))

(fn `UserConstructionScript`)