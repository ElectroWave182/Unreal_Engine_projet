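; Level teleport door actor that moves the player to another level through a trigger volume.
; When conditionable, overlap by BP_P_Torso that passes CheckPawnConditions halts the pawn, flags teleportation, plays a sound and fades in a transition screen.
; After a delay, it resolves LevelName through the game instance's level map, saves and opens that level.
; A separate Openthedoor event swings the inner door with a timeline.
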(event `self.ReceiveBeginPlay`
  (`self.InitGameInstance`))

(event `self.Trigger.OnComponentBeginOverlap`
  (params (OverlappedComponent :type "PrimitiveComponent Object Reference") (OtherActor :type "Actor Object Reference") (OtherComp :type "PrimitiveComponent Object Reference") (OtherBodyIndex :type Integer) (bFromSweep :type Boolean) (SweepResult :type "HitResult Structure (by ref)"))
  (if (`self.IsConditionable`)
    (bind _asbp_p_torso (cast `/Game/Blueprints/Player/BP_P_Torso` OtherActor))
    (bind _isvalid (`self.CheckPawnConditions`))
    (if _isvalid
      (set `MovementComponent.Velocity` (0.0 0.0 0.0) (`Character.CharacterMovement` _asbp_p_torso))
      (set `/Game/Blueprints/Player/BPP_BodyPart.isInTeleportation` true _asbp_p_torso)
      (set `/Game/Blueprints/Player/BP_P_Torso.isTeleporting` true _asbp_p_torso)
      (`self.PlaySFX` "NewEnumerator4")
      (bind _returnvalue (`|CreateWidget` "/Game/Blueprints/UI/Loading/WBP_TransitionScreen.WBP_TransitionScreen_C"))
      (`UserWidget.AddToViewport` _returnvalue 0)
      (`/Game/Blueprints/UI/Loading/WBP_TransitionScreen.Fade in` _returnvalue)
      (`KismetSystemLibrary.Delay` 6.0)
      (set `/Game/Blueprints/Player/BP_P_Torso.isTeleporting` false _asbp_p_torso)
      (set `/Game/Blueprints/Player/BPP_BodyPart.isInTeleportation` false _asbp_p_torso)
      (bind _asbp_gi_ew_game_instance (cast `/Game/Blueprints/Managing/BP_GI_EwGameInstance` (`GameplayStatics.GetGameInstance`)))
      (bind _output_get (set `/Game/Blueprints/Managing/BP_GI_EwGameInstance.currentLevelName` (`BlueprintMapLibrary.Map_Find` (`/Game/Blueprints/Managing/BP_GI_EwGameInstance.LevelMap` _asbp_gi_ew_game_instance) (`self.LevelName`)) _asbp_gi_ew_game_instance))
      (`/Game/Blueprints/Managing/BP_GI_EwGameInstance.SaveGame` _asbp_gi_ew_game_instance)
      (`GameplayStatics.OpenLevel` _output_get))))

(event `Open the door`
  (bind (_direction _axe) (`Timeline|Open door` :!via `PlayFromStart`)
    (:`Update`
      (`SceneComponent.K2_SetRelativeRotation` (`self.DoorInside`) (`KismetMathLibrary.MakeRotator` 0.0 0.0 _axe) false false))))

(fn `UserConstructionScript`
  (if (not (`self.IsConditionable`))
    (`SceneComponent.K2_SetRelativeRotation` :`self` (`self.DoorInside`))))