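; BP_SoundAmbiantActor is an ambient audio actor that plays a sound cue at its location with randomized variation.
; On BeginPlay it spawns the sound at a random start time, volume and pitch, using instrument attenuation and concurrency settings.
; A self-recursive RandomizeVolume event then re-rolls volume and pitch on a delay, whose random interval is picked once at startup.
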(event `RandomizeVolume`
  (bind _dynamicaudiocomponent (`self.DynamicAudioComponent`))
  (`AudioComponent.SetVolumeMultiplier` _dynamicaudiocomponent (`KismetMathLibrary.RandomFloatInRange` 0.0 0.75))
  (`AudioComponent.SetPitchMultiplier` _dynamicaudiocomponent (`KismetMathLibrary.RandomFloatInRange` 0.9 1.0))
  (`KismetSystemLibrary.Delay` (`self.RandomIntervalForVolumeSwitch`))
  (`self.RandomizeVolume`))

(event `self.ReceiveBeginPlay`
  (bind _returnvalue (`GameplayStatics.SpawnSoundAtLocation` (`self.SoundCue`) (`self.K2_GetActorLocation`) (struct) (`KismetMathLibrary.RandomFloatInRange` 0.0 0.75) (`KismetMathLibrary.RandomFloatInRange` 0.9 1.0) (* (`SoundBase.Duration` (`self.SoundCue`)) (`KismetMathLibrary.RandomFloat`)) "/Game/Audio/Settings/Attenuation_Instruments_Settings.Attenuation_Instruments_Settings" "/Game/Audio/Settings/Concurrency_Test_Settings.Concurrency_Test_Settings"))
  (set `self.DynamicAudioComponent` _returnvalue)
  (set `self.RandomIntervalForVolumeSwitch` (`KismetMathLibrary.RandomFloatInRange` 5.0 10.0))
  (`KismetSystemLibrary.Delay` (`self.RandomIntervalForVolumeSwitch`))
  (`self.RandomizeVolume`))

(event `self.ReceiveTick`
  (params (DeltaSeconds :type "Float (single-precision)")))

(fn `UserConstructionScript`)