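; BP_NPC_Mare is the Blueprint for the mare NPC, a horse character that can switch to playing an instrument.
; StartPlayingAnim sets the skeletal mesh to the AS_ChevalPlaying animation, then creates a static mesh component at runtime and attaches it to InstrumentSocket.
; BeginPlay, overlap and Tick are unused stubs, and the construction script only calls its parent.
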(event `StartPlayingAnim`
  (`SkeletalMeshComponent.SetAnimation` (`self.SkeletalMesh`) "/Game/Assets/Animations/AS_ChevalPlaying.AS_ChevalPlaying")
  (bind _returnvalue (`AddComponent|NODE_AddStaticMeshComponent-0` :`RelativeTransform` (`KismetMathLibrary.MakeTransform` (0.0 0.0 0.0) (struct))))
  (`SceneComponent.K2_AttachToComponent` _returnvalue (`self.SkeletalMesh`) "InstrumentSocket" "KeepRelative" "KeepRelative" "KeepRelative" true))

(fn `UserConstructionScript`
  (`parent.UserConstructionScript`))