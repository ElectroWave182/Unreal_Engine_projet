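; Lion NPC Blueprint that adds an instrument-playing performance on top of its parent's behavior.
; A StartPlayingAnim event switches the skeletal mesh to the lion's playing animation.
; The same event creates a static mesh component at runtime and attaches it to the InstrumentSocket with a rotated relative offset.
; BeginPlay and the construction script only call the parent, and Tick is disabled.
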(event `self.ReceiveBeginPlay`
  (`parent.ReceiveBeginPlay`))

(event `StartPlayingAnim`
  (`SkeletalMeshComponent.SetAnimation` (`self.SkeletalMesh`) "/Game/Assets/Animations/AS_LionPlaying.AS_LionPlaying")
  (bind _returnvalue (`AddComponent|NODE_AddStaticMeshComponent-1` :`bManualAttachment` true :`RelativeTransform` (`KismetMathLibrary.MakeTransform` (0.0 0.0 0.0) (struct :`Yaw` -90.0))))
  (`SceneComponent.K2_AttachToComponent` _returnvalue (`self.SkeletalMesh`) "InstrumentSocket" "KeepRelative" "KeepRelative" "KeepRelative" true))

(fn `UserConstructionScript`
  (`parent.UserConstructionScript`))