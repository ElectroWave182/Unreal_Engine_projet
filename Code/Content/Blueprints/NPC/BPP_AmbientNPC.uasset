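; Ambient NPC Blueprint that shows a random line of dialogue when something overlaps its trigger zone.
; On overlap begin it sets Talking, writes a random entry from Sentences into its WB_AmbientDialogue widget component and makes it visible.
; On overlap end it hides the widget but leaves Talking set.
; The Talk event is empty, and leftover viewport-widget nodes are disconnected.
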(event `Talk`)

(event `self.ReceiveBeginPlay`)

(event `self.TriggerZone.OnComponentBeginOverlap`
  (params (OverlappedComponent :type "PrimitiveComponent Object Reference") (OtherActor :type "Actor Object Reference") (OtherComp :type "PrimitiveComponent Object Reference") (OtherBodyIndex :type Integer) (bFromSweep :type Boolean) (SweepResult :type "HitResult Structure (by ref)"))
  (set `self.talking` true)
  (bind _aswb_ambient_dialogue (cast `/Game/Blueprints/UI/Dialogues/WB_AmbientDialogue` (`WidgetComponent.GetUserWidgetObject` (`self.Widget`))))
  (bind _output_get (set `/Game/Blueprints/UI/Dialogues/WB_AmbientDialogue.Full Text` (`KismetArrayLibrary.Array_Random` (`self.sentences`)) _aswb_ambient_dialogue))
  (`TextBlock.SetText` (`/Game/Blueprints/UI/Dialogues/WB_AmbientDialogue.Ambient_text` _aswb_ambient_dialogue) (`KismetTextLibrary.Conv_StringToText` _output_get))
  (`SceneComponent.SetVisibility` (`self.Widget`) true false))

(event `self.TriggerZone.OnComponentEndOverlap`
  (params (OverlappedComponent :type "PrimitiveComponent Object Reference") (OtherActor :type "Actor Object Reference") (OtherComp :type "PrimitiveComponent Object Reference") (OtherBodyIndex :type Integer))
  (`SceneComponent.SetVisibility` (`self.Widget`) false false))

(fn `UserConstructionScript`)