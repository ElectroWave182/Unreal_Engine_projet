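; NPC dialogue component that steps through a branching conversation from the DialogueData table, showing each line in a WB_Dialogue widget.
; StartTalk displays the current row, sets its animation, and picks the first child whose condition flag in the game instance is met.
; Row triggers update those flags, letting lines change later branches.
; Ending a conversation releases BP_P_Torso from dialogue and can show a one-time HUD tutorial pop-up.
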(event `self.ReceiveBeginPlay`
  (bind _asbp_gi_ew_game_instance (cast `/Game/Blueprints/Managing/BP_GI_EwGameInstance` (`GameplayStatics.GetGameInstance`)))
  (set `self.InstanceGame` _asbp_gi_ew_game_instance))

(event `Start Talk`
  (bind _referencedui (`self.referencedUI`))
  (bind _referencedui_2 (`self.referencedUI`))
  (bind _returnvalue (`GameplayStatics.GetActorOfClass` "/Game/Blueprints/Player/BP_P_Torso.BP_P_Torso_C"))
  (set `/Game/Blueprints/Player/BPP_BodyPart.IsInDialog` true _returnvalue)
  (bind _returnvalue_2 (`|GetDataTableRow` (`self.DialogueData`) (`KismetStringLibrary.Conv_StringToName` (`KismetStringLibrary.Conv_IntToString` (`self.CurrentID`))))
    (:`then`
      (`/Engine/EditorBlueprintResources/StandardMacros.IsValid` _referencedui
        (:`Is Valid`
          (if (`/Game/Blueprints/UI/Dialogues/WB_Dialogue.Is Speaking` _referencedui)
            _
            (elif (`KismetSystemLibrary.IsValid` (`/Game/Blueprints/UI/Dialogues/WB_Dialogue.TalkText` (`self.referencedUI`)))
              (bind (_id _id_children _condition _texte _trigger _animation) (break `/Game/Blueprints/NPC/S_Dialogue` _returnvalue_2))
              (bind _output_get (set `self.CurrentID` _id))
              (if (< (`.MaxValue` (`KismetMathLibrary.MaxOfIntArray` _id_children)) _output_get)
                (bind _returnvalue_3 (`GameplayStatics.GetActorOfClass` "/Game/Blueprints/Player/BP_P_Torso.BP_P_Torso_C" :!label _label))
                (set `/Game/Blueprints/Player/BPP_BodyPart.IsInDialog` false _returnvalue_3)
                (`/Engine/EditorBlueprintResources/StandardMacros.IsValid` _referencedui_2
                  (:`Is Valid`
                    (if (`self.IsPopUpDialogue`)
                      (`self.DialoguePopUpManager`))
                    (`Widget.RemoveFromParent` _referencedui_2)
                    (set `/Game/Blueprints/Player/BP_P_Torso.isRotatingDialog` false _returnvalue_3)
                    (`/Game/Blueprints/Player/BP_P_Torso.EndDialog` _returnvalue_3)
                    (bind _returnvalue_4 (`KismetMathLibrary.Conv_ByteToInt` _trigger))
                    (`self.UpdateTrig` _returnvalue_4)
                    (`self.NextDialogue` _id_children)))
                (elif (== (`KismetStringLibrary.Len` (`KismetTextLibrary.GetTextSourceString` _texte)) 1)
                  (goto _label)
                  (else
                    (`Widget.RemoveFromParent` (`self.referencedUI`))
                    (`self.UpdateTrig` _returnvalue_4 :!label _label_2)
                    (`self.NextDialogue` _id_children)
                    (bind _returnvalue_5 (`|CreateWidget` "/Game/Blueprints/UI/Dialogues/WB_Dialogue.WB_Dialogue_C" (`GameplayStatics.GetPlayerController` 0) (`self.talkSpeed`) (`KismetTextLibrary.Conv_TextToString` _texte) null))
                    (bind _output_get_2 (set `self.referencedUI` _returnvalue_5))
                    ; Setting Animation For Line
                    (set `self.AnimationEnum` _animation)
                    (`UserWidget.AddToViewport` _output_get_2 0))))
              (else
                (goto _label_2)))))
        (:`Is Not Valid`
          (goto _label_2))))))

(event `Cancel Talk`
  (bind _referencedui (`self.referencedUI`))
  (`/Engine/EditorBlueprintResources/StandardMacros.IsValid` _referencedui
    (:`Is Valid`
      (if (`KismetSystemLibrary.IsValid` (`/Game/Blueprints/UI/Dialogues/WB_Dialogue.TalkText` _referencedui))
        (`Widget.RemoveFromParent` (`self.referencedUI`))
        (bind _returnvalue (`GameplayStatics.GetActorOfClass` "/Game/Blueprints/Player/BP_P_Torso.BP_P_Torso_C"))
        (set `/Game/Blueprints/Player/BPP_BodyPart.IsInDialog` false _returnvalue)))))

(fn `DialoguePopUpManager`
  (bind _dialoguerow (`self.DialogueRow`))
  (bind _tutorialdatabollean (`/Game/Blueprints/Managing/BP_GI_EwGameInstance.TutorialDataBollean` (`self.InstanceGame`)))
  (bind _asbp_ewhud (cast `/Game/Blueprints/Managing/BP_EWHUD` (`PlayerController.GetHUD` (`GameplayStatics.GetPlayerController` 0))))
  (if (not (`BlueprintMapLibrary.Map_Find` _tutorialdatabollean _dialoguerow))
    (`/Game/Blueprints/Managing/BP_EWHUD.ShowTutorial` _asbp_ewhud _dialoguerow)
    (`BlueprintMapLibrary.Map_Add` _tutorialdatabollean _dialoguerow true)))

(fn `NextDialogue`
  (params (Childrens :type "Array of Integer"))
  (locals (oldID :type Integer))
  (if (== (`KismetArrayLibrary.Array_Length` Childrens) 0)
    (bind _returnvalue (`GameplayStatics.GetActorOfClass` "/Game/Blueprints/Player/BP_P_Torso.BP_P_Torso_C"))
    (set `/Game/Blueprints/Player/BPP_BodyPart.IsInDialog` false _returnvalue)
    (else
      (for _array_element Childrens
        (bind _returnvalue_2 (`|GetDataTableRow` (`self.DialogueData`) (`KismetStringLibrary.Conv_StringToName` (`KismetStringLibrary.Conv_IntToString` _array_element)))
          (:`then`
            (bind (_id _id_children _condition) (break `/Game/Blueprints/NPC/S_Dialogue` _returnvalue_2))
            (bind _returnvalue_3 (`KismetMathLibrary.Conv_ByteToInt` _condition))
            (if (or (`|GetArrayItem` (`/Game/Blueprints/Managing/BP_GI_EwGameInstance.DialogueConditions` (`self.InstanceGame`)) _returnvalue_3) (== _returnvalue_3 0))
              (set `self.CurrentID` _id)
              (break))))))))

(fn `SetAnimationToPlay`)

(fn `UpdateTrig`
  (params (Trigger :type Integer))
  (bind _dialogueconditions (`/Game/Blueprints/Managing/BP_GI_EwGameInstance.DialogueConditions` (`self.InstanceGame`)))
  (if (and (< Trigger 10) (> Trigger 5))
    (`KismetArrayLibrary.Array_Set` _dialogueconditions (- Trigger 5))
    (else
      (`KismetArrayLibrary.Array_Set` _dialogueconditions Trigger true))))