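; BPP_NPC is a talkable NPC that turns its mesh toward the player while they stand in its trigger zone.
; Entering the zone switches the HUD through the game instance; leaving cancels dialogue and restores that HUD.
; Talk, or entry when IsAnnoying (one-shot), starts BPACDialogue and timeline-rotates the player and camera toward the NPC.
; The construction script applies configurable mesh, animation and look-at height.
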(event `self.ReceiveTick`
  (params (DeltaSeconds :type "Float (single-precision)"))
  (bind _skeletalmesh (`self.SkeletalMesh`))
  (bind (_returnvalue_roll _returnvalue_pitch _returnvalue_yaw) (`KismetMathLibrary.BreakRotator` (`KismetMathLibrary.FindLookAtRotation` (`self.K2_GetActorLocation`) (`self.K2_GetActorLocation` (`self.torso`)))))
  ;[0 0.09757 0.15 0.5] NPC facing Player Logic
  (if (`self.dontFollow`)
    _
    (elif (`self.lookAt`)
      (`SceneComponent.K2_SetWorldRotation` (`self.SkeletalMesh`) (`KismetMathLibrary.RInterpTo` (`SceneComponent.K2_GetComponentRotation` _skeletalmesh) (`KismetMathLibrary.MakeRotator` 0.0 0.0 (+ _returnvalue_yaw -90.0)) DeltaSeconds 10.0) false false)
      (else
        (`SceneComponent.K2_SetWorldRotation` _skeletalmesh (`KismetMathLibrary.RInterpTo` (`SceneComponent.K2_GetComponentRotation` (`self.SkeletalMesh`)) (`self.initRotation`) DeltaSeconds 10.0) false false)))))

(event `self.ReceiveBeginPlay`
  ;[0 0.09757 0.15 0.5] NPC facing Player Logic
  (set `self.initRotation` (`SceneComponent.K2_GetComponentRotation` (`self.SkeletalMesh`))))

(event `self.Trigger Zone.OnComponentBeginOverlap`
  (params (OverlappedComponent :type "PrimitiveComponent Object Reference") (OtherActor :type "Actor Object Reference") (OtherComp :type "PrimitiveComponent Object Reference") (OtherBodyIndex :type Integer) (bFromSweep :type Boolean) (SweepResult :type "HitResult Structure (by ref)"))
  (bind _returnvalue (`GameplayStatics.GetPlayerController` 0))
  (bind _torso (`self.torso`))
  (bind (_returnvalue_x _returnvalue_y _returnvalue_z) (`KismetMathLibrary.BreakVector` (`SceneComponent.K2_GetComponentLocation` (`self.LookAtCamera`))))
  (bind (_returnvalue_roll _returnvalue_pitch _returnvalue_yaw) (`KismetMathLibrary.BreakRotator` (`KismetMathLibrary.FindLookAtRotation` (`self.K2_GetActorLocation` _torso) (`self.K2_GetActorLocation`))))
  ;[0 0.02554 0.15 0.5] When overlaping change player UI
  (bind _asbp_p_torso (cast `/Game/Blueprints/Player/BP_P_Torso` OtherActor))
  (bind _asbp_gi_ew_game_instance (cast `/Game/Blueprints/Managing/BP_GI_EwGameInstance` (`GameplayStatics.GetGameInstance`)))
  (`/Game/Blueprints/Managing/BP_GI_EwGameInstance.ToggleHudInGameInstance` _asbp_gi_ew_game_instance "NewEnumerator6" self _asbp_p_torso)
  (set `self.lookAt` true)
  ;[0.15 0 0 0.5] If is annoying, talk to you directly (no player interaction)
  (set `self.torso` _asbp_p_torso)
  (if (`self.isAnnoying`)
    (set `self.isAnnoying` false)
    (set `/Game/Blueprints/Player/BPP_BodyPart.IsInDialog` true _torso :!label _label)
    (if (`/Game/Blueprints/Player/BP_P_Torso.isRotatingDialog` _torso)
      ;[0.15 0.1475 0 0.5] We go in BPA_C_Dialogue PWIOUUUU
      (`/Game/Blueprints/NPC/BPA_C_Dialogue.Start Talk` (`self.BPA_C_Dialogue`) :!label _label_2)
      (else
        (set `/Game/Blueprints/Player/BP_P_Torso.isRotatingDialog` true _torso)
        (`|ExecutionSequence`
          (:`then_0`
            (goto _label_2))
          (:`then_1`
            ;[0.15 0 0 0.5] Change player rotation to face the NPC it's here if you want to make it smooth
            (bind _output_get (set `self.actualPlayerRotation` (`self.K2_GetActorRotation` _torso)))
            (bind _output_get_2 (set `self.actualControlRotation` (`Controller.GetControlRotation` _returnvalue)))
            (bind (_direction _alpha) (`Timeline|SmoothRotate` :!via `PlayFromStart`)
              (:`Update`
                (bind (_returnvalue_roll_2 _returnvalue_pitch_2 _returnvalue_yaw_2) (`KismetMathLibrary.BreakRotator` (`KismetMathLibrary.RLerp` _output_get (`KismetMathLibrary.MakeRotator` 0.0 0.0 _returnvalue_yaw) _alpha true)))
                (`self.K2_SetActorRotation` _torso (`KismetMathLibrary.MakeRotator` 0.0 0.0 _returnvalue_yaw_2) false)
                (`Controller.SetControlRotation` _returnvalue (`KismetMathLibrary.RLerp` _output_get_2 (`KismetMathLibrary.FindLookAtRotation` (`self.K2_GetActorLocation` (`self.torso`)) (`KismetMathLibrary.MakeVector` _returnvalue_x _returnvalue_y _returnvalue_z)) _alpha true))))))))))

(event `/Game/Blueprints/UI/Dialogues/BPI_Dialogue.Talk`
  (goto _label))

(event `/Game/Blueprints/UI/Dialogues/BPI_Dialogue.Cancel`)

(event `self.Trigger Zone.OnComponentEndOverlap`
  (params (OverlappedComponent :type "PrimitiveComponent Object Reference") (OtherActor :type "Actor Object Reference") (OtherComp :type "PrimitiveComponent Object Reference") (OtherBodyIndex :type Integer))
  ;[0 0.02073 0.15 0.5] On empeche l'interraction coté joueur en retirant les indications visuelles et on fait en sorte que le npc arrête de le suivre du regard
  (`/Game/Blueprints/NPC/BPA_C_Dialogue.Cancel Talk` (`self.BPA_C_Dialogue`))
  (set `self.lookAt` false)
  (bind _asbp_gi_ew_game_instance (cast `/Game/Blueprints/Managing/BP_GI_EwGameInstance` (`GameplayStatics.GetGameInstance`)))
  (if (`|EnumEquality` (`/Game/Blueprints/Managing/BP_GI_EwGameInstance.ECurrentHud` _asbp_gi_ew_game_instance) "NewEnumerator6")
    (`/Game/Blueprints/Managing/BP_GI_EwGameInstance.ToggleHudInGameInstance` _asbp_gi_ew_game_instance (`/Game/Blueprints/Managing/BP_GI_EwGameInstance.EOldHud` _asbp_gi_ew_game_instance) self null)))

(fn `UserConstructionScript`
  (bind _skeletalmesh (`self.SkeletalMesh`))
  (bind _in_animation_mode (`self.In Animation Mode`))
  (`SkeletalMeshComponent.SetSkeletalMeshAsset` (`self.SkeletalMesh`) (`self.New Mesh`))
  (`SkeletalMeshComponent.SetAnimationMode` _skeletalmesh _in_animation_mode true)
  (if (`|EnumEquality` _in_animation_mode "AnimationBlueprint")
    (`SkeletalMeshComponent.SetAnimInstanceClass` _skeletalmesh (`self.New Class`))
    (else
      (set `SkeletalMeshComponent.AnimationData` (make `SingleAnimationPlayData` (`self.AnimSequence to Play`)) _skeletalmesh)))
  (`SceneComponent.K2_SetRelativeLocation` (`self.LookAtCamera`) (`KismetMathLibrary.MakeVector` 0.0 0.0 (`self.heigthToLookAt`)) false false))