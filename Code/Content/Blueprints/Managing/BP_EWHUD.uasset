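; BP_EWHUD is a HUD Blueprint that creates the game's main HUD widget and controls its tutorial popup.
; On BeginPlay it adds WBP_MainHUD to the viewport and stores it in the game instance as MainHUDWidget.
; ShowTutorial passes a row name to the popup, reveals it and refreshes its rich-text description.
; HideTutorial collapses the popup and prints a debug string.
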(event `self.ReceiveBeginPlay`
  (bind _returnvalue (`|CreateWidget` "/Game/Blueprints/UI/HUD/WBP_MainHUD.WBP_MainHUD_C" (`GameplayStatics.GetPlayerController` 0)))
  (bind _output_get (set `self.Ref_MainHUD` _returnvalue))
  (`UserWidget.AddToViewport` _output_get 0)
  (bind _asbp_gi_ew_game_instance (cast `/Game/Blueprints/Managing/BP_GI_EwGameInstance` (`GameplayStatics.GetGameInstance`)))
  (set `/Game/Blueprints/Managing/BP_GI_EwGameInstance.mainHUDWidget` _returnvalue _asbp_gi_ew_game_instance))

(event `ShowTutorial`
  (params (TutorialRow :type Name))
  (bind _wbp_popuptuto (`/Game/Blueprints/UI/HUD/WBP_MainHUD.WBP_PopupTuto` (`self.Ref_MainHUD`)))
  (set `/Game/Blueprints/UI/HUD/WBP_PopupTuto.RowName` TutorialRow _wbp_popuptuto)
  (`Widget.SetVisibility` _wbp_popuptuto "Visible")
  (`/Game/Blueprints/UI/HUD/WBP_PopupTuto.Set Description Rich Text` _wbp_popuptuto))

(event `HideTutorial`
  (`Widget.SetVisibility` (`/Game/Blueprints/UI/HUD/WBP_MainHUD.WBP_PopupTuto` (`self.Ref_MainHUD`)) "Collapsed")
  (`KismetSystemLibrary.PrintString` "HIDE"))

(fn `UserConstructionScript`)