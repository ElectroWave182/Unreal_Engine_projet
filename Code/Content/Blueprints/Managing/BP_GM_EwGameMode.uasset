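; Game mode that runs level startup and gates player control.
; BeginPlay has the game instance switch level music and refresh parts, then builds a dialogue-condition array from the enum, with only AlwaysTrue set.
; The transition-screen fade-out, wrapped in a timed play lock, hangs off that loop's body.
; Helper events toggle the torso pawn's cinematic flag and fade in an audio component's volume through a timeline.
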(event `self.ReceiveBeginPlay`
  (bind _asbp_gi_ew_game_instance (cast `/Game/Blueprints/Managing/BP_GI_EwGameInstance` (`GameplayStatics.GetGameInstance`)))
  (bind _returnvalue (`GameplayStatics.GetCurrentLevelName` true))
  (`/Game/Blueprints/Managing/BP_GI_EwGameInstance.Switch2DMusic` _asbp_gi_ew_game_instance _returnvalue)
  (`/Game/Blueprints/Managing/BP_GI_EwGameInstance.RefreshAllParts` _asbp_gi_ew_game_instance)
  ; Create an array with needed size for E_Condition_Dialogue (First item is AlwaysTrue)
  (set `self.DialogueConditions` (`|MakeArray` true))
  (bind _enumvalue (foreach `/Game/Blueprints/NPC/E_Condition_Dialogue` false)
    (:`LoopBody`
      (if (!= _enumvalue 0)
        (`KismetArrayLibrary.Array_Add` (`self.DialogueConditions`))
        (bind _returnvalue_2 (`|CreateWidget` "/Game/Blueprints/UI/Loading/WBP_TransitionScreen.WBP_TransitionScreen_C" null 0.0))
        (`UserWidget.AddToViewport` _returnvalue_2 0)
        (`self.Disable play`)
        (`/Game/Blueprints/UI/Loading/WBP_TransitionScreen.Fade out` _returnvalue_2)
        (`KismetSystemLibrary.Delay` 1.0)
        (`self.Allow play`)))))

(event `Allow play`
  ; DESACTIVER/ACTIVER CONTROLES MURIN
  (bind _asbp_p_torso (cast `/Game/Blueprints/Player/BP_P_Torso` (`GameplayStatics.GetPlayerCharacter` 0)))
  (set `/Game/Blueprints/Player/BPP_BodyPart.IsInCinematic` false _asbp_p_torso))

(event `FadeInAudio`
  (params (AudioComp :type "AudioComponent Object Reference"))
  (bind (_direction _newtrack_0) (`Timeline|FadeInTimeline` :!via `PlayFromStart`)
    (:`Update`
      (`AudioComponent.SetVolumeMultiplier` AudioComp _newtrack_0))))

(event `Disable play`
  ; DESACTIVER/ACTIVER CONTROLES MURIN
  (bind _asbp_p_torso (cast `/Game/Blueprints/Player/BP_P_Torso` (`GameplayStatics.GetPlayerCharacter` 0)))
  (set `/Game/Blueprints/Player/BPP_BodyPart.IsInCinematic` true _asbp_p_torso))

(fn `UserConstructionScript`
  (`parent.UserConstructionScript`))