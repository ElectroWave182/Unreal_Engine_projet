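; BP_Single_Instrument_Manager is a placed audio source for one instrument type.
; On BeginPlay it looks up that type's sound cue in the game instance and spawns it at the actor's location with instrument attenuation and concurrency settings, without auto-destroy.
; If the game instance's InstrumentMap flag for that type is false, it sets the volume to zero, so the sound is still spawned but silent.
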(event `self.ReceiveBeginPlay`
  (bind _instrumenttype (`self.InstrumentType`))
  (bind _asbp_gi_ew_game_instance (cast `/Game/Blueprints/Managing/BP_GI_EwGameInstance` (`GameplayStatics.GetGameInstance`)))
  (bind _output_get (set `self.GameInstance` _asbp_gi_ew_game_instance))
  (bind _returnvalue (`GameplayStatics.SpawnSoundAtLocation` (`BlueprintMapLibrary.Map_Find` (`/Game/Blueprints/Managing/BP_GI_EwGameInstance.MapInstrumentCues` _output_get) _instrumenttype) (`self.K2_GetActorLocation`) (struct) 1.2 1.0 0.0 "/Game/Audio/Settings/Attenuation_Instruments_Settings.Attenuation_Instruments_Settings" "/Game/Audio/Settings/Concurrency_Test_Settings.Concurrency_Test_Settings" false))
  (bind _output_get_2 (set `self.AudioComp` _returnvalue))
  (if (not (`BlueprintMapLibrary.Map_Find` (`/Game/Blueprints/Managing/BP_GI_EwGameInstance.Instrument Map` _output_get) _instrumenttype))
    (`AudioComponent.SetVolumeMultiplier` _output_get_2 0.0)))

(fn `UserConstructionScript`)