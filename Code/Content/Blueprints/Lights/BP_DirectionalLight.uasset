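; Directional light actor that publishes its direction, color and intensity to the CustomLightData0 material parameter collection for custom lighting.
; Construction script and BeginPlay write the negated forward vector and the color with intensity in alpha, picking parameters by name-list index.
; When hidden, it writes only the color RGB, without direction or intensity.
; Tick is empty, so neither updates per frame.
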(event `self.ReceiveBeginPlay`
  (bind _customlightdata_0 (`self.CustomLightData_0`))
  (bind (_lightcolor_r _lightcolor_g _lightcolor_b) (break `LinearColor` (`self.LightColor`)))
  (bind _returnvalue (`MaterialParameterCollection.GetVectorParameterNames` _customlightdata_0))
  (bind _output (`|GetArrayItem` _returnvalue 2))
  (if (`self.bHidden`)
    (`KismetMaterialLibrary.SetVectorParameterValue` _customlightdata_0 _output (make `LinearColor` _lightcolor_r _lightcolor_g _lightcolor_b))
    (else
      (`KismetMaterialLibrary.SetVectorParameterValue` _customlightdata_0 (`|GetArrayItem` _returnvalue) (`KismetMathLibrary.Conv_VectorToLinearColor` (* (`KismetMathLibrary.GetForwardVector` (`self.K2_GetActorRotation`)) -1)))
      (`KismetMaterialLibrary.SetVectorParameterValue` _customlightdata_0 _output (make `LinearColor` _lightcolor_r _lightcolor_g _lightcolor_b (`self.LightIntensity`))))))

(event `self.ReceiveTick`
  (params (DeltaSeconds :type "Float (single-precision)")))

(fn `UserConstructionScript`
  (bind _customlightdata_0 (`self.CustomLightData_0`))
  (bind (_lightcolor_r _lightcolor_g _lightcolor_b) (break `LinearColor` (`self.LightColor`)))
  (bind _returnvalue (`MaterialParameterCollection.GetVectorParameterNames` _customlightdata_0))
  (bind _output (`|GetArrayItem` _returnvalue 2))
  (if (`self.bHidden`)
    (`KismetMaterialLibrary.SetVectorParameterValue` _customlightdata_0 _output (make `LinearColor` _lightcolor_r _lightcolor_g _lightcolor_b))
    (else
      (`KismetMaterialLibrary.SetVectorParameterValue` _customlightdata_0 (`|GetArrayItem` _returnvalue) (`KismetMathLibrary.Conv_VectorToLinearColor` (* (`KismetMathLibrary.GetForwardVector` (`self.K2_GetActorRotation`)) -1)))
      (`KismetMaterialLibrary.SetVectorParameterValue` _customlightdata_0 _output (make `LinearColor` _lightcolor_r _lightcolor_g _lightcolor_b (`self.LightIntensity`))))))