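; Manager for custom BP_PointLight actors that caps how many are used and limits per-frame updates to those nearest the player.
; On construction and BeginPlay it gathers the lights, logs any excess over the limit, assigns indices, updates each and zeroes unused slots in the CustomLightData parameter collection.
; Each Tick selection-sorts them by distance to the player, or world origin without one, then updates only the first MaxDynamicLights.
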(event `self.ReceiveBeginPlay`
  (`self.GetAllPointLights`)
  (`self.SortByDistanceToVector` (`self.allPointLights`)))

(event `self.ReceiveTick`
  (params (DeltaSeconds :type "Float (single-precision)"))
  (bind _returnvalue (`GameplayStatics.GetPlayerCharacter` 0))
  (bind _allpointlights (`self.allPointLights`))
  ; Les lights les plus proches du Murin sont toujours les premieres dans l'Array
  (if (`KismetSystemLibrary.IsValid` _returnvalue)
    (`self.SortByDistanceToVector` _allpointlights (`self.K2_GetActorLocation` _returnvalue))
    (else
      (`self.SortByDistanceToVector` _allpointlights)))
  ; On Update seulement les MaxDynamicLights premieres
  (for _index (range (`self.MaxDynamicLights`))
    (`/Game/Blueprints/Lights/BP_PointLight.UpdatePointLight` (`|GetArrayItem` (`self.allPointLights`) _index))))

(fn `GetAllPointLights`
  (bind _allpointlights (`self.allPointLights`))
  (bind _customlightdata (`self.CustomLightData`))
  (bind _maxlights (`self.MaxLights`))
  (bind _allpointlights_2 (`self.allPointLights`))
  (bind _returnvalue (`MaterialParameterCollection.GetVectorParameterNames` _customlightdata))
  (bind _outactors (`GameplayStatics.GetAllActorsOfClass` "/Game/Blueprints/Lights/BP_PointLight.BP_PointLight_C"))
  (set `self.allPointLights` _outactors)
  (bind _returnvalue_2 (`KismetArrayLibrary.Array_Length` _outactors))
  (if (> _returnvalue_2 (`self.MaxLights`))
    ; Error if more than 10 lights used
    (for _index (range 10 (+ (- _returnvalue_2 2) 1))
      (`KismetArrayLibrary.Array_Remove` _allpointlights _index))
    (`KismetArrayLibrary.Array_Resize` _allpointlights 10)
    (`KismetSystemLibrary.LogString` (`KismetTextLibrary.Conv_TextToString` (`|FormatText` "Only {MaxLights} are allowed! There are {NbLights} too many!" _maxlights (- _returnvalue_2 _maxlights)))))
  (for (_array_element _array_index) _allpointlights_2
    (set `/Game/Blueprints/Lights/BPP_Light.index` _array_index _array_element)
    (`/Game/Blueprints/Lights/BP_PointLight.UpdatePointLight` _array_element))
  (for _index_2 (range (`KismetArrayLibrary.Array_Length` _allpointlights_2) 10)
    (bind _returnvalue_3 (* _index_2 2))
    (`KismetMaterialLibrary.SetVectorParameterValue` _customlightdata (`|GetArrayItem` _returnvalue _returnvalue_3) (`KismetMathLibrary.Conv_VectorToLinearColor` (0.0 0.0 0.0)))
    (`KismetMaterialLibrary.SetVectorParameterValue` _customlightdata (`|GetArrayItem` _returnvalue (+ _returnvalue_3 1)) (make `LinearColor` 0.0))))

(fn `PrintActorsDistanceToVector`
  (params (InActorArray :type "Array of Actor Object Reference") (Vector :type "Vector Structure"))
  (for (_array_element _array_index) InActorArray
    (`KismetSystemLibrary.PrintString` (`KismetTextLibrary.Conv_TextToString` (`|FormatText` "{Index}: {ActorName}'s Distance={Location}" _array_index (`KismetSystemLibrary.GetDisplayName` _array_element) (`KismetMathLibrary.Vector_Distance` (`self.K2_GetActorLocation` _array_element) Vector))))))

(fn `SortByDistanceToVector`
  (params (ActorArray :type "Array of Actor Object Reference") (Vector :type "Vector Structure"))
  (locals (n :type Integer) (MinIndex :type Integer) (InActorArray :type "Array of Actor Object Reference") (TempRef :type "Actor Object Reference") (InVector :type "Vector Structure"))
  (bind _invector (`local.InVector`))
  ;[0.15 0.15 0.15 0.5 50] SelectionSort, a passer en C++ si lent
  (set `local.InVector` Vector)
  (set `local.n` (- (`KismetArrayLibrary.Array_Length` ActorArray) 1))
  (for _index (range (`local.n`))
    (set `local.MinIndex` _index)
    (for _index_2 (range (+ _index 1) (+ (`local.n`) 1))
      (if (< (`KismetMathLibrary.Vector_Distance` (`self.K2_GetActorLocation` (`|GetArrayItem` ActorArray _index_2)) _invector) (`KismetMathLibrary.Vector_Distance` (`self.K2_GetActorLocation` (`|GetArrayItem` ActorArray (`local.MinIndex`))) _invector))
        (set `local.MinIndex` _index_2)))
    (set `local.TempRef` (`|GetArrayItem` ActorArray _index))
    (`KismetArrayLibrary.Array_Set` ActorArray _index (`|GetArrayItem` ActorArray (`local.MinIndex`)))
    (`KismetArrayLibrary.Array_Set` ActorArray (`local.MinIndex`) (`local.TempRef`))))

(fn `UserConstructionScript`
  (`self.GetAllPointLights`))