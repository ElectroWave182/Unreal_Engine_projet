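; BP_PointLight is a switchable custom point light that writes its data to the CustomLightData material parameter collection.
; Its Index selects two vector parameters, one for location and one for color with intensity in alpha.
; Signal plays or reverses a timeline based on State, fading intensity between zero and LightIntensity.
; Construction calls GetAllPointLights on BP_LightManager and applies full intensity when State is on.
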(event `/Game/Blueprints/Interactive/Interfaces/BPI_ReceiveSignal.ReceiveSignal`
  ; Receive signal
  (`self.UpdateLightIntensity`))

(event `UpdateLightIntensity`
  ; Switch between light on and light off
  (if (`self.state`)
    (bind (_direction _lightevolution) (`Timeline|Intensity` :`NewTime` 1.0 :!label _label)
      (:`Update`
        (set `self.LightActualIntensity` (`KismetMathLibrary.Lerp` 0.0 (`self.LightIntensity`) _lightevolution))
        (`self.UpdatePointIntensity`)))
    (else
      (goto _label :!via `Reverse`))))

(event `SetTimeIntensity`
  ; Switch between light on and light off
  (goto _label :!via `SetNewTime`))

(event `self.ReceiveBeginPlay`
  ; If active, reverse timeline
  (if (`self.state`)
    (`self.SetTimeIntensity`)))

(fn `UpdatePointIntensity`
  (bind _customlightdata (`self.CustomLightData`))
  (bind (_lightcolor_r _lightcolor_g _lightcolor_b) (break `LinearColor` (`self.LightColor`)))
  (`KismetMaterialLibrary.SetVectorParameterValue` _customlightdata (`|GetArrayItem` (`MaterialParameterCollection.GetVectorParameterNames` _customlightdata) (+ (* (`self.index`) 2) 1)) (make `LinearColor` _lightcolor_r _lightcolor_g _lightcolor_b (`self.LightActualIntensity`))))

(fn `UpdatePointLight`
  (`self.UpdatePointLocation`)
  (`self.UpdatePointIntensity`))

(fn `UpdatePointLocation`
  (bind _customlightdata (`self.CustomLightData`))
  (`KismetMaterialLibrary.SetVectorParameterValue` _customlightdata (`|GetArrayItem` (`MaterialParameterCollection.GetVectorParameterNames` _customlightdata) (* (`self.index`) 2)) (`KismetMathLibrary.Conv_VectorToLinearColor` (`self.K2_GetActorLocation`))))

(fn `UserConstructionScript`
  (bind _returnvalue (`GameplayStatics.GetActorOfClass` "/Game/Blueprints/Lights/BP_LightManager.BP_LightManager_C"))
  (`/Engine/EditorBlueprintResources/StandardMacros.IsValid` _returnvalue
    (:`Is Valid`
      (`/Game/Blueprints/Lights/BP_LightManager.GetAllPointLights` _returnvalue)
      (if (`self.state`)
        (set `self.LightActualIntensity` (`self.LightIntensity`))
        (`self.UpdatePointIntensity`)))))