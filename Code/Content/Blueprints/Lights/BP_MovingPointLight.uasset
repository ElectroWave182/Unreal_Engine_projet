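; Moving point light that slides between its starting world location and a relative offset when it receives a signal.
; Signal optionally updates intensity, then plays or reverses a position timeline based on State, lerping the actor and refreshing the point location.
; BeginPlay sets the timeline rate to Speed divided by the length of actor location minus the offset, not the travel distance.
; Construction applies fixed intensity when ChangeIntensity is off.
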(event `/Game/Blueprints/Interactive/Interfaces/BPI_ReceiveSignal.ReceiveSignal`
  ; Receive signal
  (if (`self.changeIntensity`)
    (`self.UpdateLightIntensity`))
  (`self.UpdatePosition`))

(event `self.ReceiveBeginPlay`
  (set `self.originWorldLocation` (`self.K2_GetActorLocation`))
  (`self.UpdateSpeed`))

(event `UpdatePosition`
  (bind _originworldlocation (`self.originWorldLocation`))
  (if (`self.state`)
    (bind (_direction _lightposition) (`Timeline|LightPosition` :!label _label)
      (:`Update`
        (`self.K2_SetActorLocation` (`KismetMathLibrary.VLerp` _originworldlocation (+ _originworldlocation (`self.goToRelativeLocation`)) _lightposition))
        (`self.UpdatePointLocation`)))
    (else
      (goto _label :!via `Reverse`))))

(fn `UpdateSpeed`
  ; Update speed
  (`TimelineComponent.SetPlayRate` (`self.LightPosition`) (/ (`self.Speed`) (`KismetMathLibrary.VSize` (- (`self.K2_GetActorLocation`) (`self.goToRelativeLocation`))))))

(fn `UserConstructionScript`
  (`parent.UserConstructionScript`)
  (if (not (`self.changeIntensity`))
    (set `self.LightActualIntensity` (`self.LightIntensity`))
    (`self.UpdatePointIntensity`)))