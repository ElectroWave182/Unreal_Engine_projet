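; BP_AmbientLight is an actor that drives custom ambient lighting values through the CustomAmbientLightData0 Material Parameter Collection.
; It writes its AmbientIntensity and AmbientPower variables into the collection's first two scalar parameters, looked up by index rather than by literal name.
; The Construction Script applies the values when the actor is constructed, and BeginPlay repeats the same writes when play starts.
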(event `self.ReceiveBeginPlay`
  (bind _customambientlightdata_0 (`self.CustomAmbientLightData_0`))
  (bind _returnvalue (`MaterialParameterCollection.GetScalarParameterNames` _customambientlightdata_0))
  (`KismetMaterialLibrary.SetScalarParameterValue` _customambientlightdata_0 (`|GetArrayItem` _returnvalue) (`self.AmbientIntensity`))
  (`KismetMaterialLibrary.SetScalarParameterValue` _customambientlightdata_0 (`|GetArrayItem` _returnvalue 1) (`self.AmbientPower`)))

(fn `UserConstructionScript`
  (bind _customambientlightdata_0 (`self.CustomAmbientLightData_0`))
  (bind _returnvalue (`MaterialParameterCollection.GetScalarParameterNames` _customambientlightdata_0))
  (`KismetMaterialLibrary.SetScalarParameterValue` _customambientlightdata_0 (`|GetArrayItem` _returnvalue) (`self.AmbientIntensity`))
  (`KismetMaterialLibrary.SetScalarParameterValue` _customambientlightdata_0 (`|GetArrayItem` _returnvalue 1) (`self.AmbientPower`)))